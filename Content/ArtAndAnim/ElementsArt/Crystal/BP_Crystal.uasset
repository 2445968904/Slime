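; BP_Crystal is a crystal actor that can light up, go dark and reassemble from scattered pieces.
; Construction sets the light color and cell materials, then randomly scatters the cells by BrokeFactor; MergeEvent uses a timeline to lerp them back to origin.
; LightUp and LightOut toggle the point light, sparks and material rotation speed.
; While Target is valid, Tick feeds its location and direction offset to the FXChain effect.
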(event Custom|LightOut
  (Components|Activation|SetActive (Variables|Default|GetFX_CrystalSparks) false false)
  (Rendering|Material|SetScalarParameterValueonMaterials (Variables|Default|Getcrystal) "RotateSpeed" 0.0))

(event Custom|LightUp
  (Components|Activation|SetActive (Variables|Default|GetPointLight) true false)
  (Rendering|Material|SetScalarParameterValueonMaterials (Variables|Default|Getcrystal) "RotateSpeed" 0.2))

(event Custom|MergeEvent
  (bind _新建轨道_0 (Timeline|时间轴 PlayFromStart)
    (:Update
      (for _array_element (Variables|Default|GetCellsArray)
        (Transformation|SetRelativeLocation _array_element (Math|Vector|Lerp(Vector) (Variables|/Script/Engine.SceneComponent|GetRelativeLocation _array_element) "0, 0, 0" _新建轨道_0) false false)))))

(event EventBeginPlay)

(event Collision|EventActorBeginOverlap
  (params (OtherActor :type Actor%20Object%20Reference)))

(event EventTick
  (params (DeltaSeconds :type Float%20%28single-precision%29))
  (bind _fx_chain (Variables|Default|GetFX_Chain))
  (bind _target (Variables|Default|GetTarget))
  (bind _returnvalue (Transformation|GetActorLocation _target))
  (Utilities|IsValid (Variables|Default|GetTarget)
    (:Is%20Valid
      (Effects|Components|ParticleSystem|SetVectorParameter _fx_chain "TargetLocation" _returnvalue)
      (Effects|Components|ParticleSystem|SetVectorParameter _fx_chain "ForceLocation" (- _returnvalue (Transformation|GetActorLocation))))))

(fn ConstructionScript
  (Rendering|Components|Light|SetLightColor (Variables|Default|GetPointLight) (Variables|Default|GetNew%20Light%20Color) true)
  (bind _output_get (Variables|Default|SetCellsArray (Components|GetChildrenComponents (Variables|Default|Getcells) false)))
  (for _array_element _output_get
    (bind _as静态网格体组件 (Utilities|Casting|CastToStaticMeshComponent _array_element))
    (Rendering|Material|SetMaterial _as静态网格体组件 0 (Variables|Default|GetMaterial))
    (CallFunction|Broke)))

(fn Merge
  (for _array_element (Variables|Default|GetCellsArray)
    (Transformation|SetRelativeLocation _array_element "0, 0, 0" false false)))

(fn Broke
  (bind _brokefactor (Variables|Default|GetBrokeFactor))
  (for _array_element (Variables|Default|GetCellsArray)
    (Transformation|SetRelativeLocation _array_element "0, 0, 0" false false)
    (Transformation|AddLocalOffset _array_element (Math|Vector|MakeVector (* (Math|Random|RandomFloatinRange -5e+01 5e+01) _brokefactor) (* (Math|Random|RandomFloatinRange -5e+01 5e+01) _brokefactor) (* (Math|Random|RandomFloatinRange 0.0 1e+02) _brokefactor)) false false)))