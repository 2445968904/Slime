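; BP_GrowingVine is a procedural vine actor built entirely in the construction script, with no runtime growth logic in its graph.
; It rebuilds a spline with evenly spaced rising points, randomly jittered in X and Y on each construction.
; Each point spawns a narrowed, manually attached SplineMeshComponent spanning from the previous point to the current one.
; Points and tangents use world space, so the shape ignores the actor's transform.
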(event EventBeginPlay)

(event Collision|EventActorBeginOverlap
  (params (OtherActor :type Actor%20Object%20Reference)))

(event EventTick
  (params (DeltaSeconds :type Float%20%28single-precision%29)))

(fn ConstructionScript
  (bind _returnvalue (Math|Random|RandomFloatinRange -5e+01 5e+01))
  (bind _spline (Variables|Default|GetSpline))
  (Spline|ClearSplinePoints _spline true)
  (for _index (range 0 10)
    (Spline|AddSplinePoint _spline (Math|Vector|MakeVector _returnvalue _returnvalue (Math|Conversions|ToFloat(Integer) (* _index 100))) "World" true)
    (bind _returnvalue_2 (AddComponent|AddSplineMeshComponent true (Math|Transform|MakeTransform "0, 0, 0" "0, 0, 0" "0.200000,0.200000,1.000000")))
    (SplineMesh|SetStartandEnd _returnvalue_2 (.Location (Spline|GetLocationandTangentatSplinePoint _spline (- _index 1) "World")) (.Tangent (Spline|GetLocationandTangentatSplinePoint _spline (- _index 1) "World")) (.Location (Spline|GetLocationandTangentatSplinePoint _spline _index "World")) (.Tangent (Spline|GetLocationandTangentatSplinePoint _spline _index "World")) true :!class /Script/Engine.SplineMeshComponent)))