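; BP_PoisonToxicGooSpray is an actor that displays a configurable poison or toxic goo spray effect.
; Its construction script passes the Color, Velocity and Lifetime variables into the matching named parameters of its particle system component.
; It also applies RenderSortOrder as the particle system's translucent sort priority.
; The event graph holds only disabled placeholder events, so it adds no gameplay logic.
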(event EventBeginPlay)

(event Collision|EventActorBeginOverlap
  (params (OtherActor :type Actor%20Object%20Reference)))

(event EventTick
  (params (DeltaSeconds :type Float%20%28single-precision%29)))

(fn ConstructionScript
  ;[1 1 1] Setup the Spray Color, Velocity, and Lifetime
  (Effects|Components|ParticleSystem|SetColorParameter (Variables|Default|GetParticleSystem) "Color" (Variables|Particles|GetColor))
  (Rendering|SetTranslucentSortPriority (Variables|Default|GetParticleSystem) (Variables|Particles|GetRender%20Sort%20Order))
  (Effects|Components|ParticleSystem|SetVectorParameter (Variables|Default|GetParticleSystem) "Velocity" (Variables|Particles|GetVelocity))
  (Effects|Components|ParticleSystem|SetFloatParameter (Variables|Default|GetParticleSystem) "Lifetime" (Variables|Particles|GetLifetime)))