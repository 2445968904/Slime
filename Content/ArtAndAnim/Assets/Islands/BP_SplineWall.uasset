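; Spline-driven wall builder that lines a spline with rock static meshes, located under the island assets.
; The construction script spaces meshes evenly by distance, flipping each upside down with random yaw and slight roll, and applies a shared material and configurable width and thickness.
; A per-rock, index-offset sine bobbing effect gated by IsFloating exists but is disconnected, so the rocks stay static.
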(event EventBeginPlay)

(event Collision|EventActorBeginOverlap
  (params (OtherActor :type Actor%20Object%20Reference)))

(event EventTick
  (params (DeltaSeconds :type Float%20%28single-precision%29)))

(fn ConstructionScript
  (bind _relative_transform_scale_x (Variables|Default|GetRelative%20Transform%20Scale%20X))
  (bind _spline (Variables|Default|GetSpline))
  (Utilities|Array|Clear (Variables|Default|GetRockArray))
  (for _index (range 0 (Variables|Default|GetNum))
    (bind _returnvalue (AddComponent|AddStaticMeshComponent false (Math|Transform|MakeTransform (.location (Spline|GetTransformatDistanceAlongSpline _spline (* (/ (Spline|GetSplineLength _spline) (Variables|Default|GetNum)) _index) "Local" false)) (Math|Rotator|MakeRotator (Math|Random|RandomFloatinRange -5.0 5.0) 1.8e+02 (Math|Random|RandomFloatinRange 0.0 1.8e+02)) (Math|Vector|MakeVector _relative_transform_scale_x _relative_transform_scale_x (Variables|Default|GetThickness)))))
    (Rendering|Material|SetMaterial _returnvalue 0 (Variables|Default|GetMaterial))
    (Utilities|Array|Add (Variables|Default|GetRockArray) _returnvalue)))