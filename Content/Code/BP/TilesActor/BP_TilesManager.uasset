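; Tile manager actor that builds block terrain and grass from instanced mesh components, one per tile shape (planes, slides, stairs, corners, boundaries).
; LCGen lays a grid at 100-unit spacing from the Pointer component, writing material type to per-instance custom data.
; GrassGen scatters grass randomly by intensity; other helpers randomize, clear, or collect tile meshes through the Asset Registry.
; BeginPlay and construction script do nothing, so generation relies on external calls.
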(event EventBeginPlay)

(event Collision|EventActorBeginOverlap
  (params (OtherActor :type Actor%20Object%20Reference)))

(event EventTick
  (params (DeltaSeconds :type Float%20%28single-precision%29)))

(fn ConstructionScript)

(fn RandomGen
  (params (Array :type Array%20of%20Instanced%20Static%20Mesh%20Component%20Object%20References))
  (for _array_element Array
    (Components|InstancedStaticMesh|AddInstance _array_element (Math|Transform|MakeTransform (Math|Vector|MakeVector (Math|Conversions|ToFloat(Integer) (Math|Random|RandomIntegerinRange -20 20)) (Math|Conversions|ToFloat(Integer) (Math|Random|RandomIntegerinRange -20 20)) 0.0) "0, 0, 0" "1.000000,1.000000,1.000000") false)))

(fn GetAssetTiles
  (bind (_outassetdata _returnvalue) (Class|AssetRegistry|GetAssetsbyPath (Class|AssetRegistryHelpers|GetAssetRegistry) "/Game/ArtAndAnim/Tiles" false false))
  (if _returnvalue
    (for _array_element _outassetdata
      (bind _as静态网格体 (Utilities|Casting|CastToStaticMesh (Class|AssetRegistryHelpers|GetAsset _array_element)))
      (Utilities|Array|Add (Variables|Default|GetTilesStaticMeshArray) _as静态网格体))))

(fn MakeComponentArray
  (Utilities|Array|Clear (Variables|Default|GetTilesTypeArray))
  (return (Utilities|Array|MakeArray (Variables|Default|Getblock_prc_Plane_boundary) (Variables|Default|Getblock_prc_Slide) (Variables|Default|Getblock_prc_Slide_Corner) (Variables|Default|Getblock_prc_Slide_Boundary) (Variables|Default|Getblock_prc_Slide_Half) (Variables|Default|Getblock_prc_Slide_Half_Corner) (Variables|Default|Getblock_prc_Stairs) (Variables|Default|Getblock_prc_Stairs_Corner) (Variables|Default|Getblock_prc_Plane) (Variables|Default|GetGrass_Inst))))

(fn LCGen
  (params (Instance :type Instanced%20Static%20Mesh%20Component%20Object%20Reference) (lines :type Integer) (Column :type Integer) (Instance%20Transform%20Rotation%20Z%20%28Yaw%29 :type Float%20%28single-precision%29) (MatType :type Float%20%28double-precision%29) (StartLocation :type Vector) (Instance%20Transform%20Scale :type Vector))
  (bind _pointer (Variables|Default|Getpointer))
  (bind _relativelocation (Variables|/Script/Engine.SceneComponent|GetRelativeLocation _pointer))
  (Utilities|IsValid Instance
    (:Is%20Valid
      (for _index (range 0 lines)
        (for _index_2 (range 0 Column)
          (bind _returnvalue (Components|InstancedStaticMesh|AddInstance Instance (Math|Transform|MakeTransform (Math|Vector|MakeVector (+ (.x _relativelocation) (* _index_2 100)) (+ (.y _relativelocation) (* _index 100)) (.z _relativelocation)) (Math|Rotator|MakeRotator 0.0 0.0 Instance%20Transform%20Rotation%20Z%20%28Yaw%29) Instance%20Transform%20Scale) false))
          (Components|InstancedStaticMesh|SetCustomDataValue Instance _returnvalue 0 MatType false))))))

(fn ClearAll
  (params (Instance :type Instanced%20Static%20Mesh%20Component%20Object%20Reference))
  (Components|InstancedStaticMesh|ClearInstances Instance))

(fn SpanGrass
  (params (block_Type :type Instanced%20Static%20Mesh%20Component%20Object%20Reference))
  (return))

(fn GrassGen
  (params (lines :type Integer) (Column :type Integer) (Instance%20Transform%20Rotation%20Z%20%28Yaw%29 :type Float%20%28single-precision%29) (MatType :type Float%20%28double-precision%29) (StartLocation :type Vector) (Instance%20Transform%20Scale :type Vector) (Intensity :type Float%20%28double-precision%29))
  (bind _pointer (Variables|Default|Getpointer))
  (bind _relativelocation (Variables|/Script/Engine.SceneComponent|GetRelativeLocation _pointer))
  (for _index (range 0 lines)
    (for _index_2 (range 0 Column)
      (for _index_3 (range 0 (Math|Float|Truncate (* Intensity 0.5)))
        (Components|InstancedStaticMesh|AddInstance (Variables|Default|GetGrass_Inst) (Math|Transform|MakeTransform (Math|Vector|MakeVector (+ (.x _relativelocation) (Math|Random|RandomFloatinRange 0.0 (* lines 100))) (+ (.y _relativelocation) (Math|Random|RandomFloatinRange 0.0 (* Column 100))) (.z _relativelocation)) (Math|Rotator|MakeRotator 0.0 0.0 Instance%20Transform%20Rotation%20Z%20%28Yaw%29) Instance%20Transform%20Scale) false)))))