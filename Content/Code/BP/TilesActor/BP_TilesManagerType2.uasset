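; BP_TilesManagerType2 is a tile manager actor that builds instanced static mesh components from the meshes in the ArtAndAnim/Tiles folder.
; Its construction script queries the Asset Registry for those meshes, creates one component per mesh and adds a default instance to each.
; A RandomGen helper can add instances at random XY offsets, but nothing in this graph calls it.
; BeginPlay is empty and Initialize is a stub.
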(event EventBeginPlay)

(event Collision|EventActorBeginOverlap
  (params (OtherActor :type Actor%20Object%20Reference)))

(event EventTick
  (params (DeltaSeconds :type Float%20%28single-precision%29)))

(fn ConstructionScript
  (CallFunction|GetAssetTilesArray)
  (CallFunction|MakeInstnaceComponents)
  (for _array_element (Variables|Default|GetTilesTypeArray)
    (Components|InstancedStaticMesh|AddInstance _array_element (Math|Transform|MakeTransform "0, 0, 0" "0, 0, 0" "1.000000,1.000000,1.000000") false)))

(fn RandomGen
  (params (Array :type Array%20of%20Instanced%20Static%20Mesh%20Component%20Object%20References))
  (for _array_element Array
    (Components|InstancedStaticMesh|AddInstance _array_element (Math|Transform|MakeTransform (Math|Vector|MakeVector (Math|Conversions|ToFloat(Integer) (Math|Random|RandomIntegerinRange -20 20)) (Math|Conversions|ToFloat(Integer) (Math|Random|RandomIntegerinRange -20 20)) 0.0) "0, 0, 0" "1.000000,1.000000,1.000000") false)))

(fn GetAssetTilesArray
  (bind (_outassetdata _returnvalue) (Class|AssetRegistry|GetAssetsbyPath (Class|AssetRegistryHelpers|GetAssetRegistry) "/Game/ArtAndAnim/Tiles" false false))
  (if _returnvalue
    (for _array_element _outassetdata
      (bind _as静态网格体 (Utilities|Casting|CastToStaticMesh (Class|AssetRegistryHelpers|GetAsset _array_element)))
      (Utilities|Array|Add (Variables|Default|GetTiles%20Assets%20Array) _as静态网格体))))

(fn Initialize)

(fn MakeInstnaceComponents
  (Utilities|Array|Clear (Variables|Default|GetTilesTypeArray))
  (for _array_element (Variables|Default|GetTiles%20Assets%20Array)
    (bind _returnvalue (AddComponent|AddInstancedStaticMeshComponent false))
    (Components|StaticMesh|SetStaticMesh _returnvalue _array_element)
    (Utilities|Array|Add (Variables|Default|GetTilesTypeArray) _returnvalue)))