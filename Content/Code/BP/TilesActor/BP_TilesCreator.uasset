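; BP_TilesCreator is an actor that spawns tile meshes found in the project's Tiles content folder when play begins.
; GetAssetTiles queries the Asset Registry and casts results to Static Mesh, but returns inside its loop after adding the first.
; BeginPlay gives each collected mesh its own new Instanced Static Mesh component with one randomly Y-offset instance and a debug print.
; The Construction Script holds a disconnected copy of this logic.
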(event EventBeginPlay
  (CallFunction|GetAssetTiles)
  (for _array_element (Variables|Default|GetTilesStaticMeshArray)
    (bind _returnvalue (AddComponent|AddInstancedStaticMeshComponent false))
    (Components|StaticMesh|SetStaticMesh _returnvalue _array_element)
    (Components|InstancedStaticMesh|AddInstance _returnvalue (Math|Transform|MakeTransform (Math|Vector|MakeVector 0.0 (Math|Random|RandomFloatinRange 0.0 1e+02) 0.0) "0, 0, 0" "1.000000,1.000000,1.000000") false)
    (Development|PrintString "Hello")))

(event Collision|EventActorBeginOverlap
  (params (OtherActor :type Actor%20Object%20Reference)))

(event EventTick
  (params (DeltaSeconds :type Float%20%28single-precision%29)))

(fn ConstructionScript)

(fn GetAssetTiles
  (bind (_outassetdata _returnvalue) (Class|AssetRegistry|GetAssetsbyPath (Class|AssetRegistryHelpers|GetAssetRegistry) "/Game/ArtAndAnim/Tiles" false false))
  (if _returnvalue
    (for _array_element _outassetdata
      (bind _as静态网格体 (Utilities|Casting|CastToStaticMesh (Class|AssetRegistryHelpers|GetAsset _array_element)))
      (Utilities|Array|Add (Variables|Default|GetTilesStaticMeshArray) _as静态网格体)
      (return false))))