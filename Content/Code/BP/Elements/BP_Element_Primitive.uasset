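; BP_Element_Primitive is an element actor, still in test form, built around a SlimeAttributeHelper component that holds its element and concentration.
; Helper delegates recolor TestBox for Grass, Water or Fire and show concentration on a TextRender.
; The first TestBox hit on an actor with the same helper gives it this element as a timed continued attribute.
; Reaction forwards to the target's AttributeCalculate; ForceReaction, TryToReaction and ElementDie are empty stubs.
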(event OnComponentHit(TestBox)
  (params (HitComponent :type Primitive%20Component%20Object%20Reference) (OtherActor :type Actor%20Object%20Reference) (OtherComp :type Primitive%20Component%20Object%20Reference) (NormalImpulse :type Vector :default "0, 0, 0") (Hit :type Hit%20Result%20Structure%20%28by%20ref%29))
  (bind _returnvalue (Actor|GetComponentbyClass OtherActor "/Script/Slime.SlimeAttributeHelper"))
  ;[1 1 1] just a test
  (if (not (Variables|Default|GetOnce))
    (Utilities|IsValid _returnvalue
      (:Is%20Valid
        (Class|SlimeAttributeHelper|MakeContinuedAttribute _returnvalue (Utilities|Struct|MakeSlimeAttribute (.Element (Utilities|Struct|BreakSlimeAttribute (Variables|/Script/Slime.SlimeAttributeHelper|GetNowElement (Variables|Default|GetSlimeAttributeHelper)))) 5e+01) 1e+01)
        (Variables|Default|SetOnce true)))))

(event UpdateAttributeDelegate(SlimeAttributeHelper))

(event ElementUpdateDelegate(SlimeAttributeHelper)
  (CallFunction|ElementUpdateCallBack))

(event ConcentrationUpdateDelegate(SlimeAttributeHelper)
  (CallFunction|ConcentrationUpdateCallBack))

(event EventBeginPlay)

(event Collision|EventActorBeginOverlap
  (params (OtherActor :type Actor%20Object%20Reference)))

(event EventTick
  (params (DeltaSeconds :type Float%20%28single-precision%29)))

(fn ConstructionScript)

(fn Reaction
  (params (Actor :type Actor%20Object%20Reference) (Want :type Slime%20Attribute%20Structure))
  (Class|SlimeAttributeHelper|AttributeCalculate (Actor|GetComponentbyClass Actor "/Script/Slime.SlimeAttributeHelper") Want))

(fn ForceReaction)

(fn TrytoReaction)

(fn ReduceConcentration
  (params (Float :type Float%20%28double-precision%29))
  (Variables|Default|SetElement (Utilities|Struct|MakeSlimeAttribute (.Element (Utilities|Struct|BreakSlimeAttribute (Variables|Default|GetElement))) (- (.Concentration (Utilities|Struct|BreakSlimeAttribute (Variables|Default|GetElement))) Float)))
  (if (<= (.Concentration (Utilities|Struct|BreakSlimeAttribute (Variables|Default|GetElement))) 0.0)
    (CallFunction|ElementDie)))

(fn ElementDie)

(fn ElementUpdateCallBack
  (bind _testbox (Variables|Default|GetTestBox))
  ;[1 1 1] Just a test
  (switch Utilities|FlowControl|Switch|SwitchonEElement (.Element (Utilities|Struct|BreakSlimeAttribute (Variables|/Script/Slime.SlimeAttributeHelper|GetNowElement (Variables|Default|GetSlimeAttributeHelper))))
    (:Grass
      (Rendering|Material|SetMaterial _testbox 0 "/AnimationSharing/AnimSharingGreen.AnimSharingGreen"))
    (:Water
      (Rendering|Material|SetMaterial _testbox 0 "/AnimationSharing/AnimSharingBlue.AnimSharingBlue"))
    (:Fire
      (Rendering|Material|SetMaterial _testbox 0 "/AnimationSharing/AnimSharingRed.AnimSharingRed"))))

(fn ConcentrationUpdateCallBack
  (Rendering|Components|TextRender|SetText (Variables|Default|GetTextRender) (Utilities|Text|ToText(Float) (.Concentration (Utilities|Struct|BreakSlimeAttribute (Variables|/Script/Slime.SlimeAttributeHelper|GetNowElement (Variables|Default|GetSlimeAttributeHelper)))) "HalfToEven")))