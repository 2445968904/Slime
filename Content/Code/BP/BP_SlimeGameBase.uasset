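; Level-flow manager for the slime game, handling player start placement, checkpoints and death respawns.
; On BeginPlay it fades out the loading screen, resolves the start tag from level defaults or GameInstance saves, with a one-shot entry override, then activates the matching checkpoint and camera.
; WhenDie returns the slime to its tagged PlayerStart, restoring movement, camera and Grass element.
; Both paths reset platforms; AI spawners refresh on checkpoint load and death.
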(event Custom|WhenDie
  (bind _checkpointnow (Variables|Default|GetCheckPointNow))
  (bind _camerapoint (Variables|/Game/Code/BP/SaveSystem/CheckPoint.CheckPoint_C|GetCameraPoint _checkpointnow))
  (bind _asbp_slime_base (Utilities|Casting|CastToBP_Slime_Base (Game|GetPlayerCharacter 0)))
  (Variables|Default|SetBP%20Slime%20Base _asbp_slime_base)
  (bind _transform (CallFunction|GetPlayerStart (Variables|Default|GetPlayerTag)))
  (Transformation|SetActorTransform (Variables|Default|GetBP%20Slime%20Base) _transform)
  (Variables|/Script/Engine.MovementComponent|SetVelocity (Variables|/Script/Engine.Character|GetCharacterMovement (Variables|Default|GetBP%20Slime%20Base)) "0, 0, 0")
  (Components|Movement|StopMovementImmediately (Variables|/Script/Engine.Character|GetCharacterMovement (Variables|Default|GetBP%20Slime%20Base)))
  (Utilities|FlowControl|Sequence
    (:then_0
      ;[1 1 1] Camera
      (Utilities|IsValid _checkpointnow
        (:Is%20Valid
          (Utilities|IsValid _camerapoint
            (:Is%20Valid
              (bind _asbp_slime_base_2 (Utilities|Casting|CastToBP_Slime_Base (Game|GetPlayerCharacter 0)))
              (Default|CallonAnotherObject _camerapoint _asbp_slime_base_2))))))
    (:then_1
      (Variables|/Script/Slime.SlimeAttributeHelper|SetNowElement (Variables|/Script/Slime.Slime_Base|GetSlimeAttributeHelper (Variables|Default|GetBP%20Slime%20Base)) (Utilities|Struct|MakeSlimeAttribute "Grass" 1e+02))
      (Default|NumChange (Variables|/Game/Code/BP/BP_Slime_Base.BP_Slime_Base_C|GetGameUI (Variables|Default|GetBP%20Slime%20Base)))
      (if (Class|NavMovementComponent|IsFlying (Variables|/Script/Engine.Character|GetCharacterMovement (Variables|Default|GetBP%20Slime%20Base)))
        (Default|GetDownfromWall (Variables|Default|GetBP%20Slime%20Base))))
    (:then_2
      ;[1 1 1] 关卡重置
      (CallFunction|PlatformReset)
      (CallFunction|SpawnAIandClear))))

(event Custom|SpawnAIAndClear
  (bind _outactors (Actor|GetAllActorsOfClass "/Game/Code/AI/AISpawner.AISpawner_C"))
  (for _array_element _outactors
    (Default|ClearAI _array_element)
    (Default|CreatAI _array_element)))

(event EventBeginPlay
  (bind _returnvalue (Game|GetPlayerCharacter 0))
  (bind _returnvalue_2 (Game|GetPlayerCharacter 0))
  (bind _intomaptag (Variables|Default|GetIntoMapTag))
  (CallFunction|SlimeUI)
  (CallFunction|GetMapStartName)
  (bind _transform (CallFunction|GetPlayerStart (Utilities|String|StringToName (Utilities|String|SelectString (Utilities|String|ToString(Name) _intomaptag) (Utilities|String|ToString(Name) (Variables|Default|GetPlayerTag)) (!= _intomaptag "")))))
  (Utilities|FlowControl|Sequence
    (:then_0
      (Utilities|IsValid _returnvalue_2
        (:Is%20Valid
          (Transformation|SetActorTransform _returnvalue_2 _transform))))
    (:then_1
      (bind _outactors (Actor|GetAllActorsOfClass "/Game/Code/BP/SaveSystem/CheckPoint.CheckPoint_C"))
      (bind _array_element (Utilities|Array|ForEachLoopwithBreak _outactors :!label _label)
        (:LoopBody
          (if (Utilities|Enum|Equal(Enum) (Variables|/Game/Code/BP/SaveSystem/CheckPoint.CheckPoint_C|GetTag _array_element) (Utilities|String|ToString(Name) (Variables|Default|GetPlayerTag)))
            (Variables|Default|SetCheckPointNow _array_element)
            (goto _label Break)))
        (:Completed
          (Utilities|IsValid (Variables|Default|GetCheckPointNow)
            (:Is%20Valid
              (Utilities|FlowControl|Sequence
                (:then_0
                  ;[1 1 1] 关卡重置
                  (Default|AutoActive (Variables|Default|GetCheckPointNow) _returnvalue)
                  (CallFunction|SpawnAIandClear))
                (:then_1
                  (Utilities|IsValid (Variables|/Game/Code/BP/SaveSystem/CheckPoint.CheckPoint_C|GetCameraPoint (Variables|Default|GetCheckPointNow))
                    (:Is%20Valid
                      (bind _asbp_slime_base (Utilities|Casting|CastToBP_Slime_Base _returnvalue))
                      (Default|CallonAnotherObject (Variables|/Game/Code/BP/SaveSystem/CheckPoint.CheckPoint_C|GetCameraPoint (Variables|Default|GetCheckPointNow)) _asbp_slime_base))))))
            (:Is%20Not%20Valid
              (bind _asbp_slime_base_2 (Utilities|Casting|CastToBP_Slime_Base _returnvalue_2))
              (Default|NotFindSavePoint _asbp_slime_base_2))))))
    (:then_2
      (CallFunction|PlatformReset))))

(event EventTick
  (params (DeltaSeconds :type Float%20%28single-precision%29)))

(fn ConstructionScript)

(fn GetPlayerStart
  (params (Tag :type Name))
  (bind _outactors (Actor|GetAllActorsOfClass "/Script/Engine.PlayerStart"))
  (bind _array_element (Utilities|Array|ForEachLoopwithBreak _outactors)
    (:LoopBody
      (if (== (Variables|/Script/Engine.PlayerStart|GetPlayerStartTag _array_element) Tag)
        (return (Transformation|GetActorTransform _array_element))))))

(fn PlatformReset
  (Utilities|FlowControl|Sequence
    (:then_0
      (bind _outactors (Actor|GetAllActorsOfClass "/Game/Code/BP/Parkour/MovingPlatforms/platforms/BP_Platform.BP_Platform_C"))
      (for _array_element _outactors
        (Default|ResetCall _array_element)))))

(fn SlimeUI
  (bind _returnvalue (UserInterface|CreateWidget "/Game/Maps/Begin/Transition/LoadingTransition_Widget.LoadingTransition_Widget_C"))
  (UserInterface|Viewport|AddtoViewport _returnvalue 0)
  (UserInterface|Animation|PlayAnimation _returnvalue (Variables|/Game/Maps/Begin/Transition/LoadingTransition_Widget.LoadingTransition_Widget_C|GetBlendOut _returnvalue) 0.0 1 "Forward" 1.0 false))

(fn GetMapStartName
  (bind _returnvalue (Actor|GetActorOfClass "/Game/Maps/Begin/Transition/TransitionActor.TransitionActor_C"))
  (Utilities|IsValid _returnvalue
    (:Is%20Valid
      (if (.ReturnValue (Utilities|Map|Find (Variables|Default|GetBeginTagByLevel) (Utilities|String|StringToName (Variables|/Game/Maps/Begin/Transition/TransitionActor.TransitionActor_C|GetLevel _returnvalue))))
        (Variables|Default|SetPlayerTag (Utilities|String|StringToName (.Value (Utilities|Map|Find (Variables|Default|GetBeginTagByLevel) (Utilities|String|StringToName (Variables|/Game/Maps/Begin/Transition/TransitionActor.TransitionActor_C|GetLevel _returnvalue))))))
        (bind _asslime_game_instance (Utilities|Casting|CastToSlimeGameInstance (Game|GetGameInstance)))
        (Utilities|FlowControl|Sequence
          (:then_0
            ;[1 1 1] 注释
            (if (.ReturnValue (Utilities|Map|Find (Variables|/Game/Code/UMG/Save/SlimeGameInstance.SlimeGameInstance_C|GetPlayerMapSave _asslime_game_instance) (Utilities|String|StringToName (Variables|/Game/Maps/Begin/Transition/TransitionActor.TransitionActor_C|GetLevel _returnvalue))))
              (Variables|Default|SetPlayerTag (Utilities|String|StringToName (.Value (Utilities|Map|Find (Variables|/Game/Code/UMG/Save/SlimeGameInstance.SlimeGameInstance_C|GetPlayerMapSave _asslime_game_instance) (Utilities|String|StringToName (Variables|/Game/Maps/Begin/Transition/TransitionActor.TransitionActor_C|GetLevel _returnvalue))))))
              (if (and (.ReturnValue (Utilities|Map|Find (Variables|/Game/Code/UMG/Save/SlimeGameInstance.SlimeGameInstance_C|GetPlayerShouldGo _asslime_game_instance) (Utilities|String|StringToName (Variables|/Game/Maps/Begin/Transition/TransitionActor.TransitionActor_C|GetLevel _returnvalue)))) (Utilities|Enum|NotEqual(Enum) (.Value (Utilities|Map|Find (Variables|/Game/Code/UMG/Save/SlimeGameInstance.SlimeGameInstance_C|GetPlayerShouldGo _asslime_game_instance) (Utilities|String|StringToName (Variables|/Game/Maps/Begin/Transition/TransitionActor.TransitionActor_C|GetLevel _returnvalue)))) "None"))
                (Variables|Default|SetIntoMapTag (Utilities|String|StringToName (.Value (Utilities|Map|Find (Variables|/Game/Code/UMG/Save/SlimeGameInstance.SlimeGameInstance_C|GetPlayerShouldGo _asslime_game_instance) (Utilities|String|StringToName (Variables|/Game/Maps/Begin/Transition/TransitionActor.TransitionActor_C|GetLevel _returnvalue))))))
                (Utilities|Map|Add (Variables|/Game/Code/UMG/Save/SlimeGameInstance.SlimeGameInstance_C|GetPlayerShouldGo _asslime_game_instance) (Utilities|String|StringToName (Variables|/Game/Maps/Begin/Transition/TransitionActor.TransitionActor_C|GetLevel _returnvalue)) "None")
                (else
                  (Variables|Default|SetIntoMapTag "None"))))))
        (else
          (Variables|Default|SetPlayerTag (Variables|Default|GetBeginTag) :!label _label))))
    (:Is%20Not%20Valid
      (goto _label))))