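; Box prop that a slime pawn interacts with to enter or leave a box-pushing state; the pushing movement itself is not handled here.
; Interact alternates via FlipFlop between grab and release, toggling the slime's IsPushingBox and CanJump flags.
; Grab runs up to four debug-drawn Visibility box traces along world X/Y axes.
; The first hit turns the Arrow and snaps the slime to that side's marker component.
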(event EventBeginPlay
  (|CallParentFunction) ; 此节点被禁用，将不会被调用。\n从引脚连出引线来编译功能。
)

(event Collision|EventActorBeginOverlap
  (params (OtherActor :type Actor%20Object%20Reference))
  (|CallParentFunction OtherActor) ; 此节点被禁用，将不会被调用。\n从引脚连出引线来编译功能。
)

(event EventTick
  (params (DeltaSeconds :type Float%20%28single-precision%29))
  (|CallParentFunction DeltaSeconds) ; 此节点被禁用，将不会被调用。\n从引脚连出引线来编译功能。
)

(event EventBPIInteract
  (params (InteractPawn :type Pawn%20Object%20Reference))
  (bind _returnvalue (Transformation|GetActorLocation))
  (bind _left (Variables|Default|Getleft))
  (bind _forward (Variables|Default|Getforward))
  (bind _right (Variables|Default|Getright))
  (bind _back (Variables|Default|Getback))
  (bind _arrow (Variables|Default|GetArrow))
  (bind _half_size (Variables|Default|GetHalf%20Size))
  (bind _arrow_2 (Variables|Default|GetArrow))
  (bind _returnvalue_2 (+ _returnvalue "0.000000,0.000000,100.000000"))
  (bind _asbp_slime_base (Utilities|Casting|CastToBP_Slime_Base InteractPawn))
  (Utilities|FlowControl|FlipFlop
    (:A
      (Utilities|FlowControl|Sequence
        (:then_0
          (bind _returnvalue_3 (Collision|BoxTraceByChannel _returnvalue_2 (+ _returnvalue_2 "500.000000,0.000000,0.000000") (Math|Conversions|ToVector(Float) (Variables|Default|GetHalf%20Size)) "0, 0, 0" "TraceTypeQuery1" false 0 "ForDuration" true "(R=1.000000,G=0.000000,B=0.000000,A=1.000000)" "(R=0.000000,G=1.000000,B=0.000000,A=1.000000)" 1.0))
          (if _returnvalue_3
            (Transformation|SetRelativeRotation _arrow_2 "0.000000,180.000000,0.000000" false false)
            (Transformation|SetActorLocation _asbp_slime_base (Transformation|GetWorldLocation _left) false false)
            (Transformation|SetActorRotation _asbp_slime_base (Variables|/Script/Engine.SceneComponent|GetRelativeRotation _left))
            (Variables|/Game/Code/BP/BP_Slime_Base.BP_Slime_Base_C|SetIsPushingBox _asbp_slime_base true :!label _label)
            (Variables|/Game/Code/BP/BP_Slime_Base.BP_Slime_Base_C|SetCanJump? _asbp_slime_base false)
            (else
              (bind _returnvalue_4 (Collision|BoxTraceByChannel _returnvalue_2 (+ _returnvalue_2 "0.000000,500.000000,0.000000") (Math|Conversions|ToVector(Float) (Variables|Default|GetHalf%20Size)) "0, 0, 0" "TraceTypeQuery1" false 0 "ForDuration" true "(R=1.000000,G=0.000000,B=0.000000,A=1.000000)" "(R=0.000000,G=1.000000,B=0.000000,A=1.000000)" 1.0))
              (if _returnvalue_4
                (Transformation|SetRelativeRotation _arrow_2 "0.000000,-90.000000,0.000000" false false)
                (Transformation|SetActorLocation _asbp_slime_base (Transformation|GetWorldLocation _forward) false false)
                (Transformation|SetActorRotation _asbp_slime_base (Variables|/Script/Engine.SceneComponent|GetRelativeRotation _forward))
                (goto _label)
                (else
                  (bind _returnvalue_5 (Collision|BoxTraceByChannel _returnvalue_2 (+ _returnvalue_2 "-500.000000,0.000000,0.000000") (Math|Conversions|ToVector(Float) _half_size) "0, 0, 0" "TraceTypeQuery1" false 0 "ForDuration" true "(R=1.000000,G=0.000000,B=0.000000,A=1.000000)" "(R=0.000000,G=1.000000,B=0.000000,A=1.000000)" 1.0))
                  (if _returnvalue_5
                    (Transformation|SetRelativeRotation _arrow "0, 0, 0" false false)
                    (Transformation|SetActorLocation _asbp_slime_base (Transformation|GetWorldLocation _right) false false)
                    (Transformation|SetActorRotation _asbp_slime_base (Variables|/Script/Engine.SceneComponent|GetRelativeRotation _right))
                    (goto _label)
                    (else
                      (bind _returnvalue_6 (Collision|BoxTraceByChannel _returnvalue_2 (+ _returnvalue_2 "0.000000,-500.000000,0.000000") (Math|Conversions|ToVector(Float) _half_size) "0, 0, 0" "TraceTypeQuery1" false 0 "ForDuration" true "(R=1.000000,G=0.000000,B=0.000000,A=1.000000)" "(R=0.000000,G=1.000000,B=0.000000,A=1.000000)" 1.0))
                      (if _returnvalue_6
                        (Transformation|SetRelativeRotation _arrow "0.000000,90.000000,0.000000" false false)
                        (Transformation|SetActorLocation _asbp_slime_base (Transformation|GetWorldLocation _back) false false)
                        (Transformation|SetActorRotation _asbp_slime_base (Variables|/Script/Engine.SceneComponent|GetRelativeRotation _back))
                        (goto _label)))))))))))
    (:B
      (Variables|/Game/Code/BP/BP_Slime_Base.BP_Slime_Base_C|SetIsPushingBox _asbp_slime_base false)
      (Variables|/Game/Code/BP/BP_Slime_Base.BP_Slime_Base_C|SetCanJump? _asbp_slime_base true))))

(fn ConstructionScript
  (|CallParentFunction))