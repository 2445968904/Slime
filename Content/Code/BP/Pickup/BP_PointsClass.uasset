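; BP_PointsClass is a collectible point pickup that scores for any overlapping actor with a PointComponent.
; On mesh overlap it calls PointAdd, also reducing the collector's attribute by ReduceNumber if it has a SlimeAttributeHelper.
; It then spawns a star-collect Niagara effect, destroys itself and zeroes the collector's CharacterMovement velocity.
; Random projectile-speed and gravity setup nodes exist but are disconnected.
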(event OnComponentBeginOverlap(StaticMesh)
  (params (OverlappedComponent :type Primitive%20Component%20Object%20Reference) (OtherActor :type Actor%20Object%20Reference) (OtherComp :type Primitive%20Component%20Object%20Reference) (OtherBodyIndex :type Integer) (bFromSweep :type Boolean) (SweepResult :type Hit%20Result%20Structure%20%28by%20ref%29))
  (bind _returnvalue (Actor|GetComponentbyClass OtherActor "/Script/Slime.SlimeAttributeHelper"))
  (bind _returnvalue_2 (Actor|GetComponentbyClass OtherActor "/Game/Code/BP/Component/PointComponent/PointComponent.PointComponent_C"))
  (Utilities|IsValid _returnvalue_2
    (:Is%20Valid
      (Utilities|IsValid _returnvalue
        (:Is%20Valid
          (Default|PointAdd _returnvalue_2)
          (Class|SlimeAttributeHelper|ReduceAttribute _returnvalue (Variables|Default|GetReduce%20Number)))
        (:Is%20Not%20Valid
          (Default|PointAdd _returnvalue_2)))
      (Niagara|SpawnSystematLocation "/Game/Code/BP/Pickup/FX_StarCollect.FX_StarCollect" (Transformation|GetActorLocation))
      (Actor|DestroyActor)
      (Variables|/Script/Engine.MovementComponent|SetVelocity (Actor|GetComponentbyClass OtherActor "/Script/Engine.CharacterMovementComponent") "0, 0, 0"))))

(event EventBeginPlay)

(event Collision|EventActorBeginOverlap
  (params (OtherActor :type Actor%20Object%20Reference)))

(event EventTick
  (params (DeltaSeconds :type Float%20%28single-precision%29)))

(fn ConstructionScript)