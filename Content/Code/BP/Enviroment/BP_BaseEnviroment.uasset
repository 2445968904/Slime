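; Base environment actor that applies a water element to actors inside its box volume through their slime attribute system.
; Every Tick, it runs a stationary multi-object box trace sized to BPEnviromentBox, querying Pawn and WorldDynamic objects with persistent debug drawing.
; Each hit actor with a SlimeAttributeHelper component receives AttributeCalculate with a hard-coded Water attribute, repeated every frame rather than triggered on overlap.
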(event EventBeginPlay)

(event Collision|EventActorBeginOverlap
  (params (OtherActor :type Actor%20Object%20Reference)))

(event EventTick
  (params (DeltaSeconds :type Float%20%28single-precision%29))
  (bind _bp_enviromentbox (Variables|Default|GetBP_EnviromentBox))
  (bind _returnvalue (Transformation|GetWorldLocation _bp_enviromentbox))
  (bind _outhits (Class|KismetSystemLibrary|BoxTraceMultiforObjects _returnvalue _returnvalue (* (Variables|/Script/Engine.BoxComponent|GetBoxExtent _bp_enviromentbox) 1.0) "0, 0, 0" (Utilities|Array|MakeArray "ObjectTypeQuery3" "ObjectTypeQuery2") false 0 "Persistent" true))
  (for _array_element _outhits
    (Utilities|IsValid (Actor|GetComponentbyClass (.HitActor (Collision|BreakHitResult _array_element)) "/Script/Slime.SlimeAttributeHelper")
      (:Is%20Valid
        (Class|SlimeAttributeHelper|AttributeCalculate (Actor|GetComponentbyClass (.HitActor (Collision|BreakHitResult _array_element)) "/Script/Slime.SlimeAttributeHelper") (Utilities|Struct|MakeSlimeAttribute "Water" 1.0))))))

(fn ConstructionScript)