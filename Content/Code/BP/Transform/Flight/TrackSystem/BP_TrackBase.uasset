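; Base spline track that the player's Flight pawn follows, with its own start distance and speed.
; The construction script, when enabled, or MakeConstuction builds spline mesh segments, editor-only point-index labels and places TriggerEnd at the last point.
; BeginPlay caches the pawn, sets its start distance and applies the chosen spline point type.
; EventActivateTrack makes this the pawn's current track and passes on the track speed.
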(event Custom|EventActivateTrack
  (bind _playership (Variables|Default|GetPlayerShip))
  (bind _trackspeed (Variables|Default|GetTrackSpeed))
  (Variables|/Game/Code/BP/Transform/Flight/Flight.Flight_C|SetTrackFinished (Variables|Default|GetPlayerShip) false)
  (Variables|/Game/Code/BP/Transform/Flight/Flight.Flight_C|SetCurrentTrack (Variables|Default|GetPlayerShip) self)
  (Variables|/Game/Code/BP/Transform/Flight/Flight.Flight_C|SetThisTrackSpeed _playership _trackspeed)
  (Variables|/Game/Code/BP/Transform/Flight/Flight.Flight_C|SetCurrentTrackSpeed _playership _trackspeed)
  (Variables|Default|SetTrackLocation? true))

(event EventBeginPlay
  (bind _spline (Variables|Default|GetSpline))
  (bind _spline_2 (Variables|Default|GetSpline))
  (bind _spline_3 (Variables|Default|GetSpline))
  (bind _asflight (Utilities|Casting|CastToFlight (Game|Player|GetPlayerPawn 0)))
  (bind _output_get (Variables|Default|SetPlayerShip _asflight))
  (Variables|/Game/Code/BP/Transform/Flight/Flight.Flight_C|SetDistanceAlongTrack _output_get (Variables|Default|GetStartLocation))
  (Variables|Default|SetOriginalTrackerPos (Transformation|GetWorldLocation (Variables|Default|GetPlayerTracker)))
  (switch Utilities|FlowControl|Switch|SwitchonSplinePointType (Variables|Default|GetSplinePointType)
    (:NewEnumerator0
      (for _index (range 0 (- (Spline|GetNumberOfSplinePoints _spline_3) 1))
        (Spline|SetSplinePointType _spline_3 _index "Curve" true)))
    (:NewEnumerator1
      (for _index_2 (range 0 (- (Spline|GetNumberOfSplinePoints _spline_2) 1))
        (Spline|SetSplinePointType _spline_2 _index_2 "Linear" true)))
    (:NewEnumerator2
      (for _index_3 (range 0 (- (Spline|GetNumberOfSplinePoints _spline) 1))
        (Spline|SetSplinePointType _spline _index_3 "Constant" true)))))

(event Collision|EventActorBeginOverlap
  (params (OtherActor :type Actor%20Object%20Reference)))

(event EventTick
  (params (DeltaSeconds :type Float%20%28single-precision%29)))

(fn ConstructionScript
  (if (Variables|Default|GetRuntime_Constuction)
    (CallFunction|ConstuctionThing)))

(fn ConstuctionThing
  (bind _spline (Variables|Default|GetSpline))
  (bind _spline_2 (Variables|Default|GetSpline))
  (bind _spline_3 (Variables|Default|GetSpline))
  (bind _returnvalue (Spline|GetNumberOfSplinePoints _spline_3))
  (bind _returnvalue_2 (Spline|GetNumberOfSplinePoints _spline_2))
  (Variables|Default|SetTags (Variables|Default|GetActorTags))
  (for _index (range 0 (- (Spline|GetNumberOfSplinePoints (Variables|Default|GetSpline)) 2))
    (Variables|Default|SetIndex _index)
    (bind _returnvalue_3 (AddComponent|AddSplineMeshComponent false))
    (bind _output_get (Variables|Default|SetBoundingBox _returnvalue_3))
    (Rendering|SetVisibility _output_get (Variables|Default|GetMeshVisibleInEditor) false)
    (Development|SetHiddeninGame _output_get (Variables|Default|GetMeshHiddenInGame) false)
    (Transformation|AttachComponentToComponent (Variables|Default|GetBoundingBox) (Variables|Default|GetDefaultSceneRoot) "None" "KeepRelative" "KeepRelative" "KeepRelative" true)
    (SplineMesh|SetStartandEnd (Variables|Default|GetBoundingBox) (.Location (Spline|GetLocationandTangentatSplinePoint _spline (Variables|Default|GetIndex) "Local")) (.Tangent (Spline|GetLocationandTangentatSplinePoint _spline (Variables|Default|GetIndex) "Local")) (.Location (Spline|GetLocationandTangentatSplinePoint _spline (+ (Variables|Default|GetIndex) 1) "Local")) (.Tangent (Spline|GetLocationandTangentatSplinePoint _spline (+ (Variables|Default|GetIndex) 1) "Local")) true :!class /Script/Engine.SplineMeshComponent)
    (bind _returnvalue_4 (AddComponent|AddTextRenderComponent false))
    (Transformation|SetRelativeLocation _returnvalue_4 (Spline|GetLocationatSplinePoint (Variables|Default|GetSpline) (Variables|Default|GetIndex) "Local") false true)
    (Transformation|SetRelativeRotation _returnvalue_4 "0,180.000000, 0" false false)
    (Development|SetHiddeninGame _returnvalue_4 true false)
    (Rendering|Components|TextRender|SetText _returnvalue_4 (Utilities|Text|ToText(Integer) (Variables|Default|GetIndex)))
    (Rendering|Components|TextRender|SetWorldSize _returnvalue_4 5e+02)
    (Rendering|Components|TextRender|SetTextRenderColor _returnvalue_4 (Math|Color|MakeColor 0 0 255 1)))
  (bind _returnvalue_5 (AddComponent|AddTextRenderComponent false))
  (Transformation|SetRelativeLocation _returnvalue_5 (Spline|GetLocationatSplinePoint _spline_3 _returnvalue "Local") false true)
  (Transformation|SetRelativeRotation _returnvalue_5 "0,180.000000, 0" false false)
  (Development|SetHiddeninGame _spline_3 true false)
  (Rendering|Components|TextRender|SetText _returnvalue_5 (Utilities|Text|ToText(Integer) (- _returnvalue 1)))
  (Rendering|Components|TextRender|SetWorldSize _returnvalue_5 5e+02)
  (Rendering|Components|TextRender|SetTextRenderColor _returnvalue_5 (Math|Color|MakeColor 0 0 255 1))
  (Transformation|SetWorldLocationAndRotation (Variables|Default|GetTriggerEnd) (Spline|GetLocationatSplinePoint _spline_2 _returnvalue_2 "World") (Spline|GetRotationatSplinePoint _spline_2 _returnvalue_2 "World") false true))

(fn MakeConstuction
  (CallFunction|ConstuctionThing))