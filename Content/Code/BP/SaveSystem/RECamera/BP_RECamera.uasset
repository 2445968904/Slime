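; BP_RECamera is a placed camera actor that blends to become the view target on StartFollowing, focus-tracking the player, and hands the view back on StopFollowing.
; Each tick its boom aims at the player, with optional pitch and yaw locks to preview angles.
; In Mario mode it eases to the slime's height and slides sideways by plane projection, clamped between two marker cubes.
; The construction script applies FOV, boom and preview settings.
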(event Custom|StartFollowing
  (Game|Player|SetViewTargetwithBlend (Game|GetPlayerController 0) self (Variables|Default|GetBlendTime) "VTBlend_Linear" 0.0 false)
  (Utilities|Struct|SetmembersinCameraFocusSettings (Variables|/Script/CinematicCamera.CineCameraComponent|GetFocusSettings (Variables|Default|GetCineCamera)) "Tracking" (Utilities|Struct|MakeCameraTrackingFocusSettings (Utilities|ResolveSoftReference (Game|Player|GetPlayerPawn 0)))))

(event Custom|StopFollowing
  (Game|Player|SetViewTargetwithBlend (Game|GetPlayerController 0) (Game|Player|GetPlayerPawn 0) 0.0 "VTBlend_Linear" 0.0 false))

(event EventBeginPlay
  (Utilities|Struct|SetmembersinCameraLensSettings (Variables|/Script/CinematicCamera.CineCameraComponent|GetLensSettings (Variables|Default|GetCineCamera)) (Variables|CameraControl|GetMinAperture) (Variables|CameraControl|GetMaxAperture))
  (bind _asbp_slime_base (Utilities|Casting|CastToBP_Slime_Base (Game|GetPlayerCharacter 0)))
  (Variables|Default|SetBP%20Slime%20Base _asbp_slime_base))

(event EventTick
  (params (DeltaSeconds :type Float%20%28single-precision%29))
  (bind _returnvalue (Transformation|GetActorLocation))
  (bind _returnvalue_2 (Transformation|GetActorForwardVector))
  (bind _returnvalue_3 (Transformation|GetActorLocation))
  (bind _returnvalue_4 (Game|Player|GetPlayerPawn 0))
  (bind _cameraboom (Variables|Default|GetCameraBoom))
  (bind _cameraboom_2 (Variables|Default|GetCameraBoom))
  (bind _bp_slime_base (Variables|Default|GetBP%20Slime%20Base))
  (bind _returnvalue_5 (Transformation|GetActorLocation _bp_slime_base))
  (bind _returnvalue_6 (Transformation|GetWorldLocation _cameraboom_2))
  (bind (_x _y _z) (Math|Vector|BreakVector _returnvalue_3))
  (bind _returnvalue_7 (Transformation|GetActorLocation _returnvalue_4))
  (bind _relativelocation (Variables|/Script/Engine.SceneComponent|GetRelativeLocation _cameraboom))
  (bind _returnvalue_8 (Math|Rotator|FindLookatRotation _returnvalue_6 _returnvalue_7))
  (bind _returnvalue_9 (Class|KismetMathLibrary|ProjectPointontoPlane _returnvalue_5 _returnvalue_3 _returnvalue_2))
  (bind (_x_2 _y_2 _z_2) (Math|Vector|BreakVector _returnvalue_9))
  (Utilities|IsValid (Variables|Default|GetBP%20Slime%20Base)
    (:Is%20Valid
      (Utilities|FlowControl|Sequence
        (:then_0
          (Transformation|SetRelativeRotation (Variables|Default|GetCameraBoom) (Math|Rotator|MakeRotator 0.0 (Math|Float|SelectFloat (Variables|CameraControl|GetPreviewPitch) (.pitch _returnvalue_8) (Variables|CameraControl|GetbLockPitch)) (Math|Float|SelectFloat (Variables|CameraControl|GetPreviewYaw) (.yaw _returnvalue_8) (Variables|CameraControl|GetbLockYaw))) false false))
        (:then_1
          (if (Variables|Default|GetIsMarioCamera)
            (Transformation|SetActorLocation (Math|Vector|MakeVector (.x _returnvalue) (.y _returnvalue) (Math|Interpolation|FInterpTo (.z _returnvalue) (.z (Transformation|GetActorLocation _bp_slime_base)) DeltaSeconds 3.0)) false false)
            (Transformation|SetRelativeLocation _cameraboom (Math|Vector|MakeVector (.x _relativelocation) (Math|Float|Clamp(Float) (* (.Y (Math|Vector|BreakVector (Math|Vector|ProjectVectorontoVector (Math|Vector|MakeVector (- _x_2 _x) (- _y_2 _y) (- _z_2 _z)) (Transformation|GetActorRightVector)))) -1.0) (.y (Variables|/Script/Engine.SceneComponent|GetRelativeLocation (Variables|Default|GetCubeLeft))) (.y (Variables|/Script/Engine.SceneComponent|GetRelativeLocation (Variables|Default|GetCubeRight)))) (.z _relativelocation)) false false)))))))

(fn ConstructionScript
  (bind _cubeleft (Variables|Default|GetCubeLeft))
  (Camera|SetFieldOfView (Variables|Default|GetCineCamera) (Variables|CameraControl|GetFOV))
  (LocalVariables|SetTempCameraHeightOffset (Math|Vector|MakeVector 0.0 0.0 (Variables|CameraControl|GetCameraHeight)))
  (LocalVariables|SetTempCameraRotationOffset (Math|Rotator|MakeRotator 0.0 (Variables|CameraControl|GetPreviewPitch) (Variables|CameraControl|GetPreviewYaw)))
  (Transformation|SetRelativeLocationAndRotation (Variables|Default|GetCameraBoom) (LocalVariables|GetTempCameraHeightOffset) (LocalVariables|GetTempCameraRotationOffset) false false)
  (Variables|/Script/Engine.SpringArmComponent|SetTargetArmLength (Variables|Default|GetCameraBoom) (Variables|CameraControl|GetBoomLength))
  (Variables|/Script/Engine.SpringArmComponent|SetbEnableCameraRotationLag (Variables|Default|GetCameraBoom) (Variables|CameraControl|GetbBoomRotationLag))
  (Variables|/Script/Engine.SpringArmComponent|SetCameraRotationLagSpeed (Variables|Default|GetCameraBoom) (Variables|CameraControl|GetBoomRotationLagSpeed))
  (if (Variables|Default|GetIsMarioCamera)
    (Rendering|SetVisibility _cubeleft true false)
    (Transformation|SetRelativeLocation _cubeleft (Math|Vector|MakeVector 0.0 (* (.Y (Math|Vector|BreakVector (Variables|/Script/Engine.SceneComponent|GetRelativeLocation (Variables|Default|GetCubeRight)))) -1.0) 0.0) false false)
    (else
      (Rendering|SetVisibility (Variables|Default|GetCubeLeft) false false))))