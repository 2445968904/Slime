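; Actor component that manages the active BP_RECamera for its owner and supplies camera-relative movement directions.
; CameraWantToAdd makes the passed camera current and starts it following; Close_AutoCamera blends the view back to the owner and clears it.
; CameraRelatedInput refreshes its stored camera yaw only while input is zero, so held directions survive camera cuts.
; An older distance-based camera search is disconnected, leaving BeginPlay and Tick empty.
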(event Custom|CameraWantToAdd
  (params (CameraAdd :type BP%20RE%20Camera%20Object%20Reference))
  (Variables|Default|SetTempRECamera CameraAdd)
  (Utilities|IsValid (Variables|Default|GetRECamera)
    (:Is%20Valid
      (if true
        (bind _output_get (Variables|Default|SetRECamera (Variables|Default|GetTempRECamera)))
        (Default|StartFollowing _output_get)))
    (:Is%20Not%20Valid
      (bind _output_get_2 (Variables|Default|SetRECamera (Variables|Default|GetTempRECamera)))
      (Default|StartFollowing _output_get_2))))

(event Custom|Close_AutoCamera
  (params (BlendTime :type Float%20%28single-precision%29))
  (Utilities|IsValid (Variables|Default|GetRECamera)
    (:Is%20Valid
      (Game|Player|SetViewTargetwithBlend (Game|GetPlayerController 0) (Components|GetOwner) BlendTime "VTBlend_Linear" 0.0 false)
      (Variables|Default|SetRECamera 0))))

(event EventTick
  (params (DeltaSeconds :type Float%20%28single-precision%29)))

(event EventBeginPlay)

(fn CameraRelatedInput
  (params (ForwardInput :type Float%20%28double-precision%29) (RightInput :type Float%20%28double-precision%29))
  (if (and (== ForwardInput 0.0) (== RightInput 0.0))
    (bind _output_get (Variables|Default|SetTempYaw (.yaw (Camera|GetCameraRotation (Game|GetPlayerCameraManager 0))))))
  (return (Math|Vector|GetForwardVector (Math|Rotator|MakeRotator 0.0 0.0 _output_get)) (Math|Vector|GetRightVector (Math|Rotator|MakeRotator 0.0 0.0 _output_get))))