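; BP_button is a pressure button for the parkour moving platforms that opens and closes linked actors through interface messages.
; Its box tracks overlapping actors carrying UseTag while ItemsActivated is set, so the first one in presses it and the last one out releases it.
; Pressing swaps mesh and material, messages every LinkedActor and plays a sound.
; With PressInteract set, overlaps only toggle a text prompt, as the interact toggle logic is unconnected.
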(event OnComponentBeginOverlap(Box)
  (params (OverlappedComponent :type Primitive%20Component%20Object%20Reference) (OtherActor :type Actor%20Object%20Reference) (OtherComp :type Primitive%20Component%20Object%20Reference) (OtherBodyIndex :type Integer) (bFromSweep :type Boolean) (SweepResult :type Hit%20Result%20Structure%20%28by%20ref%29))
  (bind _actor (Variables|Default|GetActor))
  (Variables|Default|SetOverlaping true)
  (if (Variables|Default|GetItemsActivated)
    (if (and (== (Utilities|Array|FindItem _actor OtherActor) -1) (Actor|ActorHasTag OtherActor (Variables|Default|GetUseTag)))
      (Utilities|FlowControl|Sequence
        (:then_0
          (if (Utilities|Array|IsEmpty (Variables|Default|GetActor))
            (CallFunction|Overlap)))
        (:then_1
          (Utilities|Array|Add _actor OtherActor))))))

(event OnComponentEndOverlap(Box)
  (params (OverlappedComponent :type Primitive%20Component%20Object%20Reference) (OtherActor :type Actor%20Object%20Reference) (OtherComp :type Primitive%20Component%20Object%20Reference) (OtherBodyIndex :type Integer))
  (bind _actor (Variables|Default|GetActor))
  (bind _actor_2 (Variables|Default|GetActor))
  (bind _returnvalue (Utilities|Array|FindItem _actor_2 OtherActor))
  (if (not (== _returnvalue -1))
    (Utilities|Array|RemoveIndex _actor _returnvalue)
    (if (Utilities|Array|IsEmpty _actor)
      (Variables|Default|SetOverlaping false)
      (CallFunction|EndOverlap))))

(event Custom|Overlap
  (bind _cube (Variables|Default|GetCube))
  (if (Variables|Default|GetPressInteract)
    (Rendering|SetVisibility (Variables|Default|GetTextRender) true false)
    (else
      (Components|StaticMesh|SetStaticMesh _cube (Variables|Default|GetPressedMesh))
      (CallFunction|EnterVol)
      (Rendering|Material|SetMaterial _cube 0 "/AnimationSharing/AnimSharingGreen.AnimSharingGreen"))))

(event Custom|EnterVol
  (for _array_element (Variables|Platfroms|GetLinkedActor)
    (Class|BPIButton|BPIOpen(Message) _array_element))
  (Audio|PlaySoundatLocation (Variables|Default|GetActiveateSound) (Transformation|GetWorldLocation (Variables|Default|GetCube self)) "0, 0, 0" 1.0 1.0 0.0 0 0 0 0)
  (Collision|SetCollisionEnabled (Variables|Default|GetBox) "QueryAndPhysics"))

(event Custom|EndOverlap
  (if (Variables|Default|GetPressInteract)
    (Rendering|SetVisibility (Variables|Default|GetTextRender) false false)
    (else
      (Components|StaticMesh|SetStaticMesh (Variables|Default|GetCube) (Variables|Default|GetUnpressedMesh))
      (CallFunction|ExitVol)
      (Rendering|Material|SetMaterial (Variables|Default|GetCube) 0 "/Game/ArtAndAnim/PolygonPrototype/props/Materials/M_Button.M_Button"))))

(event Custom|ExitVol
  (for _array_element (Variables|Platfroms|GetLinkedActor)
    (Class|BPIButton|BPIClose(Message) _array_element)))

(event EventBeginPlay
  (Rendering|SetVisibility (Variables|Default|GetTextRender) false false))

(event EventTick
  (params (DeltaSeconds :type Float%20%28single-precision%29)))

(fn ConstructionScript
  (Components|StaticMesh|SetStaticMesh (Variables|Default|GetCube) (Variables|Default|GetUnpressedMesh))
  (if (Variables|Default|GetPressInteract)
    (Rendering|SetVisibility (Variables|Default|GetTextRender) true false)
    (else
      (Rendering|SetVisibility (Variables|Default|GetTextRender) false false))))