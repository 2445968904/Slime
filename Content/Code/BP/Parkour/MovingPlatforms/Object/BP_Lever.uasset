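; Hittable lever that controls a linked spline moving platform (SplinePlat) in the parkour content.
; A hit toggles the On/Off state behind a 0.2s re-entry guard, activates or deactivates the platform, and swings the lever mesh via a timeline with a sound.
; Tick continuously sets the platform's direction from the forward/backward function configured for each state.
; The construction script applies the timeline rate and starting lever pose.
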(event Custom|LeverChange
  (params (DeltaTime :type Float%20%28double-precision%29))
  (bind _onrotation (Variables|Default|GetOnRotation))
  (bind _offrotation (Variables|Default|GetOffRotation))
  (bind _onrotation_2 (Variables|Default|GetOnRotation))
  (bind _offrotation_2 (Variables|Default|GetOffRotation))
  (bind _returnvalue (Math|Interpolation|FInterpTo _onrotation _offrotation DeltaTime 1.0))
  (bind _returnvalue_2 (Math|Interpolation|FInterpTo _offrotation_2 _onrotation_2 DeltaTime 1.0))
  (switch Utilities|FlowControl|Switch|SwitchonEnum_OnOff (Variables|Default|GetOnOff)
    (:NewEnumerator0
      (Transformation|SetRelativeRotation (Variables|Default|GetSM_lever) (Math|Rotator|MakeRotator _returnvalue_2 0.0 0.0) false false)
      (Development|PrintString (Utilities|String|ToString(Float) _returnvalue_2) true true "(R=0.000000,G=0.660000,B=1.000000,A=1.000000)" 2.0 "1"))
    (:NewEnumerator1
      (Transformation|SetRelativeRotation (Variables|Default|GetSM_lever) (Math|Rotator|MakeRotator _returnvalue 0.0 0.0) false false)
      (Development|PrintString (Utilities|String|ToString(Float) _returnvalue) true true "(R=0.000000,G=0.660000,B=1.000000,A=1.000000)" 2.0 "1"))))

(event Custom|ChangeLevel
  (if (not (Variables|Default|GetInteracted))
    (Variables|Default|SetInteracted true)
    (switch Utilities|FlowControl|Switch|SwitchonEnum_OnOff (Variables|Default|GetOnOff)
      (:NewEnumerator0
        (Variables|Default|SetOnOff "NewEnumerator1")
        (Default|Active (Variables|Default|GetsplinePlat) true))
      (:NewEnumerator1
        (Variables|Default|SetOnOff "NewEnumerator0")
        (Default|Active (Variables|Default|GetsplinePlat) false)))
    (Utilities|FlowControl|Delay 0.2)
    (Variables|Default|SetInteracted false)))

(event Custom|LeverChange_TimelineFunction
  (if (Audio|Components|Audio|IsPlaying (Variables|Default|GetTimelineLever))
    (Utilities|String|Reverse (Variables|Default|GetTimelineLever))
    (else
      (Audio|PlaySound2D "/Game/ArtAndAnim/Landscape_Final/Music/Level/拉杆sfx_Cue.拉杆sfx_Cue" 1.0 1.5 0.5 0 0)
      (switch Utilities|FlowControl|Switch|SwitchonEnum_OnOff (Variables|Default|GetOnOff)
        (:NewEnumerator0
          (bind _alpha (Timeline|TimelineLever PlayFromStart)
            (:Update
              (Transformation|SetRelativeRotation (Variables|Default|GetSM_lever) (Math|Rotator|MakeRotator (Math|Float|Lerp (Variables|Default|GetOffRotation) (Variables|Default|GetOnRotation) _alpha) 0.0 0.0) false false))))
        (:NewEnumerator1
          (Timeline|TimelineLever ReverseFromEnd))))))

(event EventBeHit
  (params (Damage :type Integer) (hitter :type Actor%20Object%20Reference))
  (CallFunction|ChangeLevel)
  (CallFunction|LeverChangeTimelineFunction))

(event EventTick
  (params (DeltaSeconds :type Float%20%28single-precision%29))
  (CallFunction|OnOffFunctions))

(fn ConstructionScript
  (Components|Timeline|SetPlayRate (Variables|Default|GetTimelineLever) (Variables|Default|GetLeverRate))
  (Rendering|SetVisibility (Variables|Default|GetTextRender) false false)
  (switch Utilities|FlowControl|Switch|SwitchonEnum_OnOff (Variables|Default|GetOnOff)
    (:NewEnumerator0
      (Transformation|SetRelativeRotation (Variables|Default|GetSM_lever) (Math|Rotator|MakeRotator (Variables|Default|GetOnRotation) 0.0 0.0) false false))
    (:NewEnumerator1
      (Transformation|SetRelativeRotation (Variables|Default|GetSM_lever) (Math|Rotator|MakeRotator (Variables|Default|GetOffRotation) 0.0 0.0) false false))))

(fn OnOffFunctions
  (bind _splineplat (Variables|Default|GetsplinePlat))
  (switch Utilities|FlowControl|Switch|SwitchonEnum_OnOff (Variables|Default|GetOnOff)
    (:NewEnumerator0
      (switch Utilities|FlowControl|Switch|SwitchonEnum_OnOffFunctions (Variables|Function|GetOnFunction)
        (:NewEnumerator1
          (Variables|/Game/Code/BP/Parkour/MovingPlatforms/platforms/BP_SplinePlatform.BP_SplinePlatform_C|SetBackForward _splineplat "NewEnumerator0"))
        (:NewEnumerator5
          (Variables|/Game/Code/BP/Parkour/MovingPlatforms/platforms/BP_SplinePlatform.BP_SplinePlatform_C|SetBackForward _splineplat "NewEnumerator1"))))
    (:NewEnumerator1
      (switch Utilities|FlowControl|Switch|SwitchonEnum_OnOffFunctions (Variables|Function|GetOffFunction)
        (:NewEnumerator1
          (Variables|/Game/Code/BP/Parkour/MovingPlatforms/platforms/BP_SplinePlatform.BP_SplinePlatform_C|SetBackForward _splineplat "NewEnumerator0"))
        (:NewEnumerator5
          (Variables|/Game/Code/BP/Parkour/MovingPlatforms/platforms/BP_SplinePlatform.BP_SplinePlatform_C|SetBackForward _splineplat "NewEnumerator1"))))))