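; BP_Platform is a parkour moving platform that activates when a Character overlaps its box and can deactivate when they leave.
; Tick moves it by a fixed per-frame offset, while a timer with optional text can kill, drop via physics, stop or teleport it to start.
; Rotation runs always or while active, optionally gated by on/off timer arrays through a DoOnce-and-Delay loop.
; With reverse enabled, leaving triggers a delayed MoveComponentTo return, interrupted by re-entry.
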(event OnComponentBeginOverlap(Box)
  (params (OverlappedComponent :type Primitive%20Component%20Object%20Reference) (OtherActor :type Actor%20Object%20Reference) (OtherComp :type Primitive%20Component%20Object%20Reference) (OtherBodyIndex :type Integer) (bFromSweep :type Boolean) (SweepResult :type Hit%20Result%20Structure%20%28by%20ref%29))
  (bind _startposition (Variables|Default|GetStartPosition))
  (Utilities|Casting|CastToCharacter OtherActor)
  (Variables|Default|SetActivated true)
  (Variables|Default|SetReverse false)
  (Components|MoveComponentTo (Variables|Default|GetPlatform) _startposition "0, 0, 0" false false (/ (Math|Vector|VectorLength (- _startposition (Transformation|GetActorLocation))) (/ (Math|Vector|VectorLength (Variables|Default|GetSpeeds)) (Utilities|Time|GetWorldDeltaSeconds))) false) ; enters at Stop
)

(event OnComponentEndOverlap(Box)
  (params (OverlappedComponent :type Primitive%20Component%20Object%20Reference) (OtherActor :type Actor%20Object%20Reference) (OtherComp :type Primitive%20Component%20Object%20Reference) (OtherBodyIndex :type Integer))
  (bind _startposition (Variables|Default|GetStartPosition))
  (Utilities|Casting|CastToCharacter OtherActor)
  (if (Variables|Default|GetDeacivateOnLeave)
    (Variables|Default|SetActivated false)
    (if (not (Variables|Default|GetReverse))
      (if (Variables|Default|GetUseReverse)
        (Variables|Default|SetReverse true)
        (Utilities|FlowControl|Delay 2.0)
        (Components|MoveComponentTo (Variables|Default|GetPlatform) _startposition "0, 0, 0" false false (/ (Math|Vector|VectorLength (- _startposition (Transformation|GetActorLocation))) (/ (Math|Vector|VectorLength (Variables|Default|GetSpeeds)) (Utilities|Time|GetWorldDeltaSeconds))) false)))))

(event Custom|StepRotation
  (bind _rotationactivetimer (Variables|rotation|GetRotationActiveTimer))
  (bind _rotationofftimer (Variables|rotation|GetRotationOffTimer))
  (Utilities|FlowControl|DoOnce false
    (:Completed
      (Utilities|FlowControl|Delay (Utilities|Array|Get(acopy) _rotationactivetimer (Variables|Rotation|GetActiveStep)))
      (if (> (Utilities|Array|Length _rotationactivetimer) 0)
        (Variables|Rotation|SetActiveStep 0)
        (else
          (Variables|Rotation|SetActiveStep (+ (Variables|Rotation|GetActiveStep) 1))))
      (Variables|Rotation|SetActivatedRotator false)
      (Utilities|FlowControl|Delay (Utilities|Array|Get(acopy) _rotationofftimer (Variables|Rotation|GetOffSetp)))
      (if (> (Variables|Rotation|GetOffSetp) (Utilities|Array|Length _rotationofftimer))
        (Variables|Rotation|SetOffSetp 0)
        (else
          (Variables|Rotation|SetOffSetp (+ (Variables|Rotation|GetOffSetp) 1))))
      (Variables|Rotation|SetActivatedRotator true)
      (CallFunction|Reset))))

(event Custom|Reset_Call
  (Variables|Default|Settimer 0.0)
  (Transformation|SetWorldLocation (Variables|Default|GetPlatform) (Variables|Default|GetStartPosition) false false)
  (Variables|Default|SetActivated false)
  (Variables|Default|SetReverse false))

(event Custom|Reset
  (bind _rotationactivetimer (Variables|rotation|GetRotationActiveTimer))
  (bind _rotationofftimer (Variables|rotation|GetRotationOffTimer))
  (Utilities|FlowControl|DoOnce false) ; enters at Reset
)

(event EventTick
  (params (DeltaSeconds :type Float%20%28single-precision%29))
  (bind _platform (Variables|Default|GetPlatform))
  (if (Variables|Default|GetDrop)
    (Physics|SetSimulatePhysics (Variables|Default|GetPlatform) true)
    (else
      (CallFunction|FuncRotations)
      (if (and (Variables|Default|GetActivated) (not (Variables|Default|GetStoped)))
        (Transformation|SetWorldLocation _platform (+ (Transformation|GetWorldLocation _platform) (Variables|Default|GetSpeeds)) false false)
        (if (Utilities|Enum|NotEqual(Enum) (Variables|Default|GetTimerFunction) "NewEnumerator0")
          (Variables|Default|Settimer (+ (Variables|Default|Gettimer) (Variables|Default|GettimerRate)))
          (CallFunction|FuncSetText)
          (if (>= (Variables|Default|Gettimer) (Variables|Default|GetLifetime))
            (switch Utilities|FlowControl|Switch|SwitchonEnum_TimerTraits (Variables|Default|GetTimerFunction)
              (:NewEnumerator1
                (Actor|DestroyActor))
              (:NewEnumerator2
                (Variables|Default|SetDrop true))
              (:NewEnumerator4
                (Variables|Default|SetStoped true))
              (:NewEnumerator5
                (Variables|Default|Settimer 0.0)
                (Transformation|SetWorldLocation (Variables|Default|GetPlatform) (Variables|Default|GetStartPosition) false false)))))
        (elif (Variables|Default|GetUseReverse)
          (if (Variables|Default|GetReverse)
            _))))))

(fn ConstructionScript
  (bind _platform (Variables|Default|GetPlatform))
  (bind _timetext (Variables|Default|GetTimeText))
  (Components|StaticMesh|SetStaticMesh _platform (Variables|Default|GetMesh))
  (Variables|Default|SetStartPosition (Transformation|GetWorldLocation _platform))
  (if (or (Utilities|Enum|Equal(Enum) (Variables|Default|GetTimerFunction) "NewEnumerator0") (not (Variables|Default|GetDisplayTimer)))
    (Rendering|SetVisibility _timetext false false)
    (else
      (Rendering|Components|TextRender|SetText _timetext (Utilities|Text|ToText(Integer) (Math|Float|Round (Variables|Default|GetLifetime)))))))

(fn FuncSetText
  (bind _timetext (Variables|Default|GetTimeText))
  (if (Variables|Default|GetDisplayTimer)
    (Rendering|SetVisibility _timetext false false)
    (else
      (Rendering|Components|TextRender|SetText _timetext (Utilities|Text|ToText(Integer) (Math|Float|Round (- (Variables|Default|GetLifetime) (Variables|Default|Gettimer))))))))

(fn FuncRotations
  (bind _activatedrotator (Variables|Rotation|GetActivatedRotator))
  (switch Utilities|FlowControl|Switch|SwitchonEnum_Rotation (Variables|Rotation|GetRotations)
    (:NewEnumerator1
      (Transformation|AddLocalRotation (Variables|Default|GetPlatform) (Variables|Rotation|GetRotationValues) false false :!label _label))
    (:NewEnumerator2
      (if (Variables|Default|GetActivated)
        (goto _label)))
    (:NewEnumerator3
      (CallFunction|StepRotation)
      (if _activatedrotator
        (goto _label)))
    (:NewEnumerator4
      (CallFunction|StepRotation)
      (if (and _activatedrotator (Variables|Default|GetActivated))
        (goto _label)))))