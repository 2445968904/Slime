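; Parkour moving platform rotator: arms spin around a central pivot, carrying platforms.
; The construction script builds arm meshes from angle and length arrays, attaching platforms at each arm's "Pivot" socket.
; Tick pitches arms continuously, when activated, or on DoOnce-gated on/off timer cycles, while each platform stays upright or spins itself.
; Overlap activation and lifetime actions (kill, drop, stop, teleport) are disconnected.
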(event OnComponentBeginOverlap(Box)
  (params (OverlappedComponent :type Primitive%20Component%20Object%20Reference) (OtherActor :type Actor%20Object%20Reference) (OtherComp :type Primitive%20Component%20Object%20Reference) (OtherBodyIndex :type Integer) (bFromSweep :type Boolean) (SweepResult :type Hit%20Result%20Structure%20%28by%20ref%29)))

(event OnComponentEndOverlap(Box)
  (params (OverlappedComponent :type Primitive%20Component%20Object%20Reference) (OtherActor :type Actor%20Object%20Reference) (OtherComp :type Primitive%20Component%20Object%20Reference) (OtherBodyIndex :type Integer)))

(event Custom|StepRotation
  (bind _rotationactivetimer (Variables|rotation|GetRotationActiveTimer))
  (bind _rotationofftimer (Variables|rotation|GetRotationOffTimer))
  (Utilities|FlowControl|DoOnce false
    (:Completed
      (Utilities|FlowControl|Delay (Utilities|Array|Get(acopy) _rotationactivetimer (Variables|Rotation|GetActiveStep)))
      (if (> (Utilities|Array|Length _rotationactivetimer) 0)
        (Variables|Rotation|SetActiveStep 0)
        (else
          (Variables|Rotation|SetActiveStep (+ (Variables|Rotation|GetActiveStep) 1))))
      (Variables|Rotation|SetActivatedRotator false)
      (Utilities|FlowControl|Delay (Utilities|Array|Get(acopy) _rotationofftimer (Variables|Rotation|GetOffSetp)))
      (if (> (Variables|Rotation|GetOffSetp) (Utilities|Array|Length _rotationofftimer))
        (Variables|Rotation|SetOffSetp 0)
        (else
          (Variables|Rotation|SetOffSetp (+ (Variables|Rotation|GetOffSetp) 1))))
      (Variables|Rotation|SetActivatedRotator true)
      (CallFunction|Reset))))

(event Custom|PlatformsRotation
  (for (_array_element _array_index) (Variables|Default|GetPlatformsMain)
    (switch Utilities|FlowControl|Switch|SwitchonEnum_ArmPlatforms (Utilities|Array|Get(acopy) (Variables|Arms|GetPlatforms) _array_index)
      (:NewEnumerator6
        (Transformation|SetWorldRotation _array_element "0, 0, 0" false false))
      (:NewEnumerator7
        (Transformation|AddLocalRotation _array_element (Math|Rotator|MakeRotator 0.0 (Utilities|Array|Get(acopy) (Variables|Arms|GetArmSpeed) _array_index) 0.0) false false)))))

(event Custom|Reset
  (bind _rotationactivetimer (Variables|rotation|GetRotationActiveTimer))
  (bind _rotationofftimer (Variables|rotation|GetRotationOffTimer))
  (Utilities|FlowControl|DoOnce false) ; enters at Reset
)

(event EventTick
  (params (DeltaSeconds :type Float%20%28single-precision%29))
  (CallFunction|PlatformsRotation)
  (CallFunction|FuncRotations DeltaSeconds)
  (if (and (Variables|Default|GetActivated) (not (Variables|Default|GetStoped)))
    (if (Utilities|Enum|NotEqual(Enum) (Utilities|Array|Get(acopy) (Variables|Default|GetTimerFunction)) "NewEnumerator0")
      (Variables|Default|Settimer (+ (Variables|Default|Gettimer) (Variables|Default|GettimerRate))))))

(fn ConstructionScript
  (for (_array_element _array_index) (Variables|Arms|GetArmRotations)
    (bind _returnvalue (AddComponent|AddStaticMeshComponent true (Math|Transform|MakeTransform (Transformation|GetWorldLocation (Variables|Default|GetPivotPoint)) (Math|Rotator|MakeRotator 0.0 _array_element 0.0) (Math|Vector|MakeVector (Utilities|Array|Get(acopy) (Variables|Arms|GetArmLengths) _array_index) 1.0 1.0))))
    (Rendering|SetCastShadow _returnvalue false)
    (Utilities|Array|SetArrayElem (Variables|Default|GetArms) _array_index _returnvalue true)
    (Transformation|AttachComponentToComponent _returnvalue (Variables|Default|GetPivotPoint) "None" "SnapToTarget" "KeepRelative" "KeepRelative" true)
    (if (Utilities|Enum|NotEqual(Enum) (Utilities|Array|Get(acopy) (Variables|Arms|GetPlatforms) _array_index) "NewEnumerator0")
      (bind _returnvalue_2 (AddComponent|AddStaticMeshComponent true (Math|Transform|MakeTransform "0, 0, 0" "0, 0, 0" (Variables|Default|GetPlatformScale))))
      (Rendering|SetCastShadow _returnvalue_2 false)
      (Utilities|Array|SetArrayElem (Variables|Default|GetPlatformsMain) _array_index _returnvalue_2 true)
      (Components|StaticMesh|SetStaticMesh _returnvalue_2 (Utilities|Array|Get(acopy) (Variables|Mesh|GetPlatFormMesh) _array_index))
      (Transformation|AttachComponentToComponent _returnvalue_2 _returnvalue "Pivot" "SnapToTarget" "KeepRelative" "KeepWorld" true))))

(fn FuncRotations
  (params (DeltaTime :type Float%20%28double-precision%29))
  (bind _activatedrotator (Variables|Rotation|GetActivatedRotator))
  (for _array_element (Variables|Default|GetArms)
    (switch Utilities|FlowControl|Switch|SwitchonEnum_Rotation (Variables|Rotation|GetRotations)
      (:NewEnumerator1
        (Transformation|AddLocalRotation _array_element (Math|Rotator|MakeRotator 0.0 (Variables|Rotation|GetRotationSpeed) 0.0) false false :!label _label))
      (:NewEnumerator2
        (if (Variables|Default|GetActivated)
          (goto _label)))
      (:NewEnumerator3
        (CallFunction|StepRotation)
        (if _activatedrotator
          (goto _label)))
      (:NewEnumerator4
        (CallFunction|StepRotation)
        (if (and _activatedrotator (Variables|Default|GetActivated))
          (goto _label))))))