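; BP_Door is a parkour door that opens once enough activation signals are active.
; Interface Open and Close events raise or lower a counter, which is compared with NeedNum to call OpenDoor or CloseDoor.
; Opening hides the static mesh and disables its collision.
; Closing switches collision to physics-only but also sets the mesh hidden, so the door never becomes visible again.
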(event Custom|Active
  (params (Active? :type Boolean))
  (if Active?
    (Math|Integer|IncrementInt (Variables|Default|GetNum)
      (:%20%20
        _))
    (else
      (Math|Integer|DecrementInt (Variables|Default|GetNum)
        (:%20%20
          _))))
  (if (>= (Variables|Default|GetNum) (Variables|Default|GetNeedNum))
    (CallFunction|OpenDoor)
    (else
      (CallFunction|CloseDoor))))

(event Custom|OpenDoor
  (bind _staticmesh (Variables|Default|GetStaticMesh))
  (Rendering|SetVisibility _staticmesh false false)
  (Collision|SetCollisionEnabled _staticmesh "NoCollision"))

(event Custom|CloseDoor
  (bind _staticmesh (Variables|Default|GetStaticMesh))
  (Rendering|SetVisibility _staticmesh false false)
  (Collision|SetCollisionEnabled _staticmesh "PhysicsOnly"))

(event EventBeginPlay)

(event Collision|EventActorBeginOverlap
  (params (OtherActor :type Actor%20Object%20Reference)))

(event EventTick
  (params (DeltaSeconds :type Float%20%28single-precision%29)))

(event EventBPIClose
  (CallFunction|Active false))

(event EventBPIOpen
  (CallFunction|Active true))

(fn ConstructionScript)