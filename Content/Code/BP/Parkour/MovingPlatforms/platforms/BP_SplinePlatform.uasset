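; Spline-following platform that shuttles between both ends of its path, optionally acting as a pressure-plate-activated mover or door.
; Construction sets the mesh and measures the spline; Tick advances a clamped distance at per-direction speeds, updating location and optional rotation.
; Endpoints flip direction, with options to wait, teleport to start or stop.
; InVolume/ExitVolume events drive activation, door direction and once-per-entry damage; the box overlap handlers are disconnected.
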(event OnComponentBeginOverlap(Box)
  (params (OverlappedComponent :type Primitive%20Component%20Object%20Reference) (OtherActor :type Actor%20Object%20Reference) (OtherComp :type Primitive%20Component%20Object%20Reference) (OtherBodyIndex :type Integer) (bFromSweep :type Boolean) (SweepResult :type Hit%20Result%20Structure%20%28by%20ref%29)))

(event OnComponentEndOverlap(Box)
  (params (OverlappedComponent :type Primitive%20Component%20Object%20Reference) (OtherActor :type Actor%20Object%20Reference) (OtherComp :type Primitive%20Component%20Object%20Reference) (OtherBodyIndex :type Integer)))

(event Custom|ExitVolume
  (Utilities|FlowControl|Sequence
    (:then_0
      (Utilities|ApplyDamage?) ; enters at Reset
    )
    (:then_1
      (if (Variables|Main|GetFunctionAsDoor)
        (Variables|Default|SetBackForward "NewEnumerator1")
        (Variables|Default|SetactiveState "NewEnumerator0")
        (else
          (Variables|Default|SetActivated false))))))

(event Custom|InVolume
  (Variables|Default|SetActivated true)
  (Utilities|ApplyDamage?
    (:output
      (if (Variables|Main|GetFunctionAsDoor)
        (Variables|Default|SetBackForward "NewEnumerator0")
        (Variables|Default|SetactiveState "NewEnumerator0")))))

(event EventTick
  (params (DeltaSeconds :type Float%20%28single-precision%29))
  (if (Utilities|Enum|Equal(Enum) (Variables|Default|GetactiveState) "NewEnumerator0")
    (if (Variables|Main|GetPressuerPlate)
      (if (Variables|Default|GetActivated)
        (if (Variables|Default|GetWait) :!label _label
          (Utilities|FlowControl|Delay (Variables|Main|GetWaitTime))
          (Variables|Default|SetWait false))
        (CallFunction|FuncSetDistance)
        (CallFunction|FuncUpdatePosition)
        (switch Utilities|FlowControl|Switch|SwitchonEnum_BackForward (Variables|Default|GetBackForward)
          (:NewEnumerator0
            (if (>= (Variables|Default|GetCurrDistance) (Variables|Default|GetDistance))
              (Variables|Default|SetBackForward "NewEnumerator1")
              (Variables|Default|SetWait true :!label _label_2)
              (if (Variables|Main|GetTeleport)
                (Variables|Default|SetCurrDistance 0.0)
                (CallFunction|FuncUpdatePosition))
              (if (Variables|Main|GetStopAtEnds)
                (Variables|Default|SetactiveState "NewEnumerator1"))))
          (:NewEnumerator1
            (if (<= (Variables|Default|GetCurrDistance) 0.0)
              (Variables|Default|SetBackForward "NewEnumerator0")
              (goto _label_2)))))
      (else
        (goto _label)))))

(fn ConstructionScript
  (bind _nodelocations (Variables|Default|GetNodeLocations))
  (bind _spline (Variables|Components|GetSpline))
  (Components|StaticMesh|SetStaticMesh (Variables|Components|GetPlatform) (Variables|Components|GetMesh))
  (Variables|Default|SetDistance (Spline|GetSplineLength (Variables|Components|GetSpline)))
  (Utilities|Array|Clear _nodelocations)
  (for _index (range 0 (Spline|GetNumberOfSplinePoints _spline))
    (Utilities|Array|Add _nodelocations (Spline|GetDistanceAlongSplineatSplinePoint _spline _index))))

(fn FuncSetDistance
  (bind _distance (Variables|Default|GetDistance))
  (switch Utilities|FlowControl|Switch|SwitchonEnum_BackForward (Variables|Default|GetBackForward)
    (:NewEnumerator0
      (Variables|Default|SetCurrDistance (Math|Float|Clamp(Float) (+ (Math|Interpolation|FInterpTo 0.0 _distance 0.01 (* (/ (Variables|Main|GetForwardSpeed) _distance) 1e+03)) (Variables|Default|GetCurrDistance)) 0.0 _distance)))
    (:NewEnumerator1
      (Variables|Default|SetCurrDistance (Math|Float|Clamp(Float) (- (Variables|Default|GetCurrDistance) (Math|Interpolation|FInterpTo 0.0 _distance 0.01 (* (/ (Variables|Main|GetBackSpeed) _distance) 1e+03))) 0.0 _distance)))))

(fn FuncUpdatePosition
  (bind _currdistance (Variables|Default|GetCurrDistance))
  (bind _spline (Variables|Components|GetSpline))
  (if (Variables|Main|GetCanRotate)
    (Transformation|SetWorldLocationAndRotation (Variables|Components|GetPlatform) (Spline|GetLocationatDistanceAlongSpline _spline _currdistance "World") (Spline|GetRotationatDistanceAlongSpline _spline _currdistance "World") false false)
    (else
      (Transformation|SetWorldLocationAndRotation (Variables|Components|GetPlatform) (Spline|GetLocationatDistanceAlongSpline (Variables|Components|GetSpline) _currdistance "World") "0, 0, 0" false false))))