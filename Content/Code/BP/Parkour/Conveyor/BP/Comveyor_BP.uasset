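; Conveyor belt actor that carries overlapping characters and tagged objects along its mesh's forward direction.
; While active, Tick adds velocity impulses to characters and offsets "convey"-tagged actors inside the Box.
; On leaving, "conveyGONew" actors get a forward nudge, and small pushable boxes optionally fall.
; Interface events start/stop the belt or rotate it 180 degrees, updating a dynamic material's scroll speed or color respectively.
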(event OnComponentEndOverlap(Box)
  (params (OverlappedComponent :type Primitive%20Component%20Object%20Reference) (OtherActor :type Actor%20Object%20Reference) (OtherComp :type Primitive%20Component%20Object%20Reference) (OtherBodyIndex :type Integer))
  (if (Actor|ActorHasTag OtherActor "conveyGONew")
    (Transformation|AddActorWorldOffset OtherActor (* (Math|Vector|GetForwardVector (Transformation|GetWorldRotation (Variables|Default|GetStaticMesh))) (* (Variables|Default|GetSpeed) 0.2)))
    (bind _aspushable_box_small (Utilities|Casting|CastToPushableBox_Small OtherActor))
    (if (Variables|Default|GetUseFall)
      (Default|FallDown _aspushable_box_small))))

(event Custom|Reverse)

(event EventBPIClose
  (Transformation|AddWorldRotation (Variables|Default|GetDefaultSceneRoot self) "0.000000,-180.000000,0.000000" false false)
  (Rendering|Material|SetVectorParameterValue (Variables|Default|GetMat) "Color" "(R=0.593750,G=0.516337,B=0.000000,A=1.000000)" :!class /Script/Engine.MaterialInstanceDynamic))

(event EventBPIOpen
  (Transformation|AddWorldRotation (Variables|Default|GetDefaultSceneRoot self) "0.000000,180.000000,0.000000" false false)
  (Rendering|Material|SetVectorParameterValue (Variables|Default|GetMat) "Color" "(R=0.000000,G=0.387657,B=1.000000,A=1.000000)" :!class /Script/Engine.MaterialInstanceDynamic))

(event EventTick
  (params (DeltaSeconds :type Float%20%28single-precision%29))
  (bind _speed (Variables|Default|GetSpeed))
  (bind _staticmesh (Variables|Default|GetStaticMesh))
  (bind _returnvalue (Transformation|GetWorldRotation _staticmesh))
  (bind _returnvalue_2 (* _speed DeltaSeconds))
  (bind _returnvalue_3 (Math|Vector|GetForwardVector _returnvalue))
  (bind _returnvalue_4 (* _returnvalue_3 _returnvalue_2))
  (if (Variables|Default|GetActive)
    (for _array_element (Collision|GetOverlappingActors (Variables|Default|GetBox) 0 :!class /Script/Engine.PrimitiveComponent)
      (bind _as角色 (Utilities|Casting|CastToCharacter _array_element)
        (:then
          (Physics|AddImpulse (Variables|/Script/Engine.Character|GetCharacterMovement _as角色) (* _returnvalue_4 5e+01) true))
        (:CastFailed
          (if (Actor|ActorHasTag _array_element "convey")
            (Transformation|AddActorWorldOffset _array_element _returnvalue_4)))))))

(event EventBPIConStop
  (Variables|Default|SetActive false)
  (Rendering|Material|SetScalarParameterValue (Variables|Default|GetMat) "XSpeed" 0.0 :!class /Script/Engine.MaterialInstanceDynamic))

(event EventBPIConBegin
  (Variables|Default|SetActive true)
  (Rendering|Material|SetScalarParameterValue (Variables|Default|GetMat) "XSpeed" (Variables|Default|GetTrackSpeed) :!class /Script/Engine.MaterialInstanceDynamic))

(fn ConstructionScript
  (bind _staticmesh (Variables|Default|GetStaticMesh))
  (bind _returnvalue (Rendering|Material|CreateDynamicMaterialInstance _staticmesh 0 "/Game/Code/BP/Parkour/Conveyor/Conveyor_M.Conveyor_M" "None" :!class /Script/Engine.PrimitiveComponent))
  (Variables|Default|SetMat _returnvalue)
  (Rendering|Material|SetMaterial _staticmesh 0 _returnvalue)
  (Rendering|Material|SetVectorParameterValue _returnvalue "Color" (Variables|Default|GetColor) :!class /Script/Engine.MaterialInstanceDynamic)
  (Rendering|Material|SetScalarParameterValue _returnvalue "XScale" (Variables|Default|GetXScale) :!class /Script/Engine.MaterialInstanceDynamic)
  (Rendering|Material|SetScalarParameterValue _returnvalue "XSpeed" (Variables|Default|GetTrackSpeed) :!class /Script/Engine.MaterialInstanceDynamic))