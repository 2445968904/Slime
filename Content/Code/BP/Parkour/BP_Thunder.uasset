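; BP_Thunder is a thunder effect actor, built from a Niagara effect and two point lights.
; Its event graph holds a looping Delay chain that waits out a dark period, activates both lights and Niagara, then switches PointLight1 off before Niagara and PointLight2.
; That chain is unconnected and never runs: BeginPlay, the construction script, ThunderBurst and ThunderClose are all empty.
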(event EventBeginPlay)

(fn ConstructionScript)

(fn ThunderBurst)

(fn ThunderClose)