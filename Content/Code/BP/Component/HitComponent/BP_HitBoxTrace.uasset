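; Hit-box trace object that detects hits from a moving box component, implementing overridable init, validity and update hooks.
; Each update sweeps multi box traces from the box's last transform to its current one, by object types and channels, using its scaled extent.
; It reports HitActors values, though the traces append only to OutHits.
; An uncalled helper interpolates points along an arc around an axis point.
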(event EventBeginPlay)

(event Collision|EventActorBeginOverlap
  (params (OtherActor :type Actor%20Object%20Reference)))

(event EventTick
  (params (DeltaSeconds :type Float%20%28single-precision%29))
  (Class|HitTraceBase|UpdateHitTrace 0.0 (Variables|Default|GetHit%20Trace%20Parameter)))

(fn ConstructionScript)

(fn ReWriteInitHitTrace
  (params (HitTraceParameter :type Hit%20Trace%20Parameter%20Structure))
  (Variables|Default|SetHit%20Trace%20Parameter HitTraceParameter)
  (Variables|Default|SetValid true)
  (return false))

(fn ReWriteIsValid
  (return (Variables|Default|GetValid)))

(fn ReWriteUpdateHitTrace
  (params (DeltaTime :type Float%20%28single-precision%29) (HitTraceParameter :type Hit%20Trace%20Parameter%20Structure))
  (bind (_hitter _hbox _traceobjecttypes _tracechannels) (Utilities|Struct|BreakHitTraceParameter HitTraceParameter))
  (if (Variables|Default|GetValid)
    (Variables|Default|SetHitBox _hbox)
    (Utilities|Array|AddUnique (Variables|Default|GetActors%20to%20Ignore) 0)
    (bind _hitresult (CallFunction|HitTrace _hitter _traceobjecttypes _tracechannels))
    (bind _values (Utilities|Map|Values _hitresult))
    (bind _output_get (Variables|Default|Setres (Utilities|Struct|MakeHitTraceResult _values)))
    (if (Utilities|Array|IsEmpty _values)
      (return _output_get false)
      (else
        (return _output_get true)))
    (else
      (return "" false))))

(fn HitTrace
  (params (Hitter :type Actor%20Object%20Reference) (ObjectTypes :type Array%20of%20EObjectTypeQuery%20Enums :default "ObjectTypeQuery1") (TraceChannel :type Array%20of%20ETraceTypeQuery%20Enums :default "TraceTypeQuery1"))
  (bind _hitbox (Variables|Default|GetHitBox))
  (bind _hitbox_2 (Variables|Default|GetHitBox))
  (bind _returnvalue (Transformation|GetWorldTransform _hitbox))
  (bind _returnvalue_2 (Transformation|GetWorldTransform _hitbox_2))
  (bind _location (Math|Transform|BreakTransform _returnvalue))
  (bind _rotation (Math|Transform|BreakTransform _returnvalue_2))
  (Variables|Default|SetObjectTypeArr ObjectTypes)
  (Utilities|FlowControl|Sequence
    (:then_0
      (for _array_element TraceChannel
        (Utilities|Array|AddUnique (LocalVariables|GetChannelArr) _array_element)))
    (:then_1
      (Variables|Default|SetHalfSize (* (Components|Box|GetScaledBoxExtent (Variables|Default|GetHitBox)) (Variables|Default|GetHit%20Box%20Scale)))
      (Utilities|FlowControl|Sequence
        (:then_0
          (if (Utilities|Array|IsNotEmpty (Variables|Default|GetObjectTypeArr))
            (bind (_outhits _returnvalue_3) (Class|KismetSystemLibrary|BoxTraceMultiforObjects (.location (Variables|Default|GetLastTransfrom)) _location (Variables|Default|GetHalfSize) _rotation (Variables|Default|GetObjectTypeArr) false (Variables|Default|GetActors%20to%20Ignore) (Variables|Default|GetObjectDraw) true "(R=1.000000,G=0.000000,B=0.000000,A=1.000000)" "(R=0.000000,G=1.000000,B=0.000000,A=1.000000)" (Variables|Default|GetDraw%20Time)))
            (if _returnvalue_3
              (Utilities|Array|AppendArray (LocalVariables|GetOutHits) _outhits))))
        (:then_1
          (for _array_element_2 (LocalVariables|GetChannelArr)
            (bind (_outhits_2 _returnvalue_4) (Class|KismetSystemLibrary|BoxTraceMulti (.location (Variables|Default|GetLastTransfrom)) _location (Variables|Default|GetHalfSize) _rotation _array_element_2 false (Variables|Default|GetActors%20to%20Ignore) (Variables|Default|GetChannel%20Draw) true "(R=1.000000,G=0.000000,B=0.000000,A=1.000000)" "(R=0.000000,G=1.000000,B=0.000000,A=1.000000)" (Variables|Default|GetDraw%20Time)))
            (if _returnvalue_4
              (Utilities|Array|AppendArray (LocalVariables|GetOutHits) _outhits_2))))))
    (:then_2
      (Variables|Default|SetLastTransfrom (Transformation|GetWorldTransform (Variables|Default|GetHitBox))))
    (:then_3
      (return (LocalVariables|GetHit%20Actors)))))

(fn GetInterpolationPosition
  (params (Start :type Vector) (End :type Vector) (axis :type Vector) (count :type Integer))
  (Variables|Default|SetDistanceStart (Math|Vector|Distance(Vector) Start End))
  (Variables|Default|SetDistanceEnd (Math|Vector|Distance(Vector) End axis))
  (Variables|Default|SetStepLength (/ 1.0 (Math|Conversions|ToFloat(Integer) (+ count 1))))
  (Utilities|Array|Add (Variables|Default|GetResult) Start)
  (for _index (range 1 count)
    (Utilities|Array|Add (Variables|Default|GetResult) (+ (* (Math|Vector|Normalize (- (Math|Vector|Lerp(Vector) Start End (* _index (Variables|Default|GetStepLength))) axis)) (Math|Float|Lerp (Variables|Default|GetDistanceStart) (Variables|Default|GetDistanceEnd) (* _index (Variables|Default|GetStepLength)))) axis)))
  (bind _returnvalue (Utilities|Array|Add (Variables|Default|GetResult) End))
  (return _returnvalue (Variables|Default|GetResult)))