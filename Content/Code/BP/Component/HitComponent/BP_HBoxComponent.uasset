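; BP_HBoxComponent is a hit box component with settings for object and channel tracing, but its event graph is currently inactive.
; BeginPlay is empty, and the trace setup is disconnected, so it never runs.
; That unused chain would spawn a BP_HitBoxTrace actor, initialize it with the component and its trace types, store it as Tracebase, and pass on debug draw settings and box extent.
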(event EventBeginPlay)