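; Slime trail maker, attached as a child actor, that spawns trail actors as the player's BP_Slime_Base moves.
; Tick accumulates travelled distance and calls UpdateTrails at fixed intervals.
; UpdateTrails sphere-traces for existing BP_SimplyDecal actors to block overlaps, then line-traces down, adding a spline point and spawning the given or default class there.
; Without ground, a forward trace spawns the default class on obstacles, rotated from the slime mesh's orientation.
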(event OnComponentHit(CollisionComponent)
  (params (HitComponent :type Primitive%20Component%20Object%20Reference) (OtherActor :type Actor%20Object%20Reference) (OtherComp :type Primitive%20Component%20Object%20Reference) (NormalImpulse :type Vector :default "0, 0, 0") (Hit :type Hit%20Result%20Structure%20%28by%20ref%29)))

(event OnComponentBeginOverlap(CollisionComponent)
  (params (OverlappedComponent :type Primitive%20Component%20Object%20Reference) (OtherActor :type Actor%20Object%20Reference) (OtherComp :type Primitive%20Component%20Object%20Reference) (OtherBodyIndex :type Integer) (bFromSweep :type Boolean) (SweepResult :type Hit%20Result%20Structure%20%28by%20ref%29)))

(event OnComponentBeginOverlap(Box)
  (params (OverlappedComponent :type Primitive%20Component%20Object%20Reference) (OtherActor :type Actor%20Object%20Reference) (OtherComp :type Primitive%20Component%20Object%20Reference) (OtherBodyIndex :type Integer) (bFromSweep :type Boolean) (SweepResult :type Hit%20Result%20Structure%20%28by%20ref%29)))

(event Custom|Update%20Trais%20Event
  (CallFunction|UpdateTrails))

(event EventBeginPlay
  (bind _asbp_slime_base (Utilities|Casting|CastToBP_Slime_Base (Game|Player|GetPlayerPawn 0)))
  (Variables|Default|SetAs%20BP%20Slime%20Base _asbp_slime_base))

(event Collision|EventActorBeginOverlap
  (params (OtherActor :type Actor%20Object%20Reference)))

(event EventTick
  (params (DeltaSeconds :type Float%20%28single-precision%29))
  (bind _as_bp_slime_base (Variables|Default|GetAs%20BP%20Slime%20Base))
  (bind _returnvalue (Transformation|GetVelocity _as_bp_slime_base))
  (bind _returnvalue_2 (Math|Vector|VectorLength _returnvalue))
  (if (>= _returnvalue_2 1e+01)
    (Utilities|FlowControl|Sequence
      (:then_0
        (bind _output_get (Variables|Default|SetCharacterMoveDistance (+ (Variables|Default|GetCharacterMoveDistance) (* _returnvalue_2 DeltaSeconds))))
        (while (>= _output_get 2e+01)
          (CallFunction|UpdateTrails)
          (Variables|Default|SetCharacterMoveDistance (- (Variables|Default|GetCharacterMoveDistance) 2e+01))))
      (:then_1
        (if (not (AI|Components|NavMovement|IsFalling (Variables|/Script/Engine.Character|GetCharacterMovement _as_bp_slime_base)))
          (Utilities|FlowControl|DoOnce false :!label _label))))
    (else
      (Utilities|Time|PauseTimerbyHandle (stale _returnvalue))
      (goto _label Reset))))

(fn ConstructionScript)

(fn UpdateTrails
  (params (class :type Actor%20Class%20Reference))
  (bind _returnvalue (Actor|GetParentActor))
  (bind _spline (Variables|Default|GetSpline))
  (bind _returnvalue_2 (Transformation|GetActorLocation _returnvalue))
  (bind _returnvalue_3 (+ _returnvalue_2 "0.000000,0.000000,-80.000000"))
  (Utilities|FlowControl|Sequence
    (:then_1
      (bind _outhits (Collision|MultiSphereTraceForObjects (+ _returnvalue_2 "0.000000,0.000000,80.000000") _returnvalue_3 5e+01 (Variables|Default|GetObject%20Types) false 0 "None"))
      (for _array_element _outhits
        (Utilities|Casting|CastToBP_SimplyDecal (.HitActor (Collision|BreakHitResult _array_element)))
        (LocalVariables|Setcanpla false))
      (if (LocalVariables|Getcanpla)
        (bind (_outhit _returnvalue_4) (Collision|LineTraceByChannel _returnvalue_2 _returnvalue_3 "TraceTypeQuery1" false 0 "None"))
        (if _returnvalue_4
          (Spline|AddSplinePoint (Variables|Default|GetSpline) (.Location (Collision|BreakHitResult _outhit)) "World" true)
          (if (Utilities|IsValidClass class)
            (LocalVariables|Settemp class)
            (else
              (LocalVariables|Settemp (LocalVariables|GetDefault))))
          (Game|SpawnActorfromClass (LocalVariables|Gettemp) (Math|Transform|MakeTransform (Spline|GetLocationatSplinePoint _spline (Spline|GetNumberOfSplinePoints _spline) "World") (Transformation|GetActorRotation (Actor|GetParentActor)) "1.000000,1.000000,1.000000") "Undefined" 0 0)
          (else
            (bind (_outhit_2 _returnvalue_5) (Collision|LineTraceByChannel (Transformation|GetActorLocation (Actor|GetParentActor)) (+ (Transformation|GetActorLocation (Actor|GetParentActor)) (* (Transformation|GetActorForwardVector (Actor|GetParentActor)) 2e+02)) "TraceTypeQuery1" false (Utilities|Array|MakeArray self (Actor|GetParentActor)) "None"))
            (if _returnvalue_5
              (bind _returnvalue_6 (Game|SpawnActorfromClass (LocalVariables|GetDefault) (Math|Transform|MakeTransform (Math|Vector|MakeVector (.X (Math|Vector|BreakVector (.Location (Collision|BreakHitResult _outhit_2)))) (.Y (Math|Vector|BreakVector (.Location (Collision|BreakHitResult _outhit_2)))) (- (.Z (Math|Vector|BreakVector (.Location (Collision|BreakHitResult _outhit_2)))) 5e+01)) (Math|Rotator|MakeRotator 0.0 0.0 0.0) "1.000000,1.000000,1.000000") "Undefined" 0 0))
              (Transformation|SetActorRotation _returnvalue_6 (Transformation|GetWorldRotation (Variables|/Script/Engine.Character|GetMesh (Variables|Default|GetAs%20BP%20Slime%20Base))))
              (Transformation|AddLocalRotation (Variables|/Script/Engine.Actor|GetRootComponent _returnvalue_6) "-90.000000,0.000000,0.000000" false false)
              (Transformation|AddWorldRotation (Variables|/Script/Engine.Actor|GetRootComponent _returnvalue_6) "0.000000,0.000000,90.000000" false false))))))))

(fn ChecktoMakeTrails)