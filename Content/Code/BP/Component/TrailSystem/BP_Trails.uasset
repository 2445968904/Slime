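; BP_Trails is a trail-recording actor that builds a spline along the ground beneath its parent actor.
; Each UpdateTrails call traces 50 units down on the Visibility channel, appends the hit location as a world-space spline point and prints the point count.
; ShowTrails draws a temporary debug sphere at the spline's end.
; Its event graph is empty, so both functions rely on external callers.
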(event EventBeginPlay)

(event Collision|EventActorBeginOverlap
  (params (OtherActor :type Actor%20Object%20Reference)))

(event EventTick
  (params (DeltaSeconds :type Float%20%28single-precision%29)))

(fn ConstructionScript)

(fn UpdateTrails
  (bind _returnvalue (Actor|GetParentActor))
  (bind _returnvalue_2 (Transformation|GetActorLocation _returnvalue))
  (bind _outhit (Collision|LineTraceByChannel _returnvalue_2 (+ _returnvalue_2 "0.000000,0.000000,-50.000000") "TraceTypeQuery1" false 0 "None"))
  (Spline|AddSplinePoint (Variables|Default|GetSpline) (.Location (Collision|BreakHitResult _outhit)) "World" true)
  (Development|PrintString (Utilities|String|ToString(Integer) (Spline|GetNumberOfSplinePoints (Variables|Default|GetSpline)))))

(fn ShowTrails
  (bind _spline (Variables|Default|GetSpline))
  (Rendering|Debug|DrawDebugSphere (Spline|GetLocationatSplinePoint _spline (Spline|GetNumberOfSplinePoints _spline) "World") 25.0 12 "(R=0.000000,G=1.000000,B=0.211823,A=1.000000)" 5.0 3.0))