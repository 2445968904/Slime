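; BP_SimplyDecal is a simple decal-like effect that scatters a random cluster of instanced meshes and animates its scale when play begins.
; The construction script adds a random number of instances to an InstancedStaticMesh, randomizing planar position, yaw and uniform scale.
; On BeginPlay a timeline float drives the uniform world scale of the whole InstancedStaticMesh component, so all instances scale together without per-instance updates.
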(event EventBeginPlay
  (bind _float (Timeline|时间轴 PlayFromStart)
    (:Update
      (Transformation|SetWorldScale3D (Variables|Default|GetInstancedStaticMesh) (* _float (Math|Vector|MakeVector 1.0 1.0 1.0))))))

(event EventTick
  (params (DeltaSeconds :type Float%20%28single-precision%29)))

(fn ConstructionScript
  (for _index (range 0 (Math|Random|RandomIntegerinRange 10 30))
    (Components|InstancedStaticMesh|AddInstance (Variables|Default|GetInstancedStaticMesh) (Math|Transform|MakeTransform (Math|Vector|MakeVector (Math|Random|RandomFloatinRange -2e+01 2e+01) (Math|Random|RandomFloatinRange -2e+01 2e+01) 0.0) (Math|Rotator|MakeRotator 0.0 0.0 (Math|Random|RandomFloatinRange -9e+01 9e+01)) (Math|Conversions|ToVector(Float) (Math|Random|RandomFloatinRange 0.5 0.6))) false)))