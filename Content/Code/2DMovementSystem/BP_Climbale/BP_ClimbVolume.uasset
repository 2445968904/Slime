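; Trigger volume that marks a wall or ladder as climbable for slime characters in the 2D movement system.
; Construction sizes the box from the parent wall or ladder dimensions.
; Overlap passes climb-through and horizontal flags to the slime's BP_Climbing component, and Tick feeds it the top height while the parent is attached.
; Attach and detach events toggle the parent's Attached flag, with detach also releasing the character.
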(event OnComponentBeginOverlap(Box)
  (params (OverlappedComponent :type Primitive%20Component%20Object%20Reference) (OtherActor :type Actor%20Object%20Reference) (OtherComp :type Primitive%20Component%20Object%20Reference) (OtherBodyIndex :type Integer) (bFromSweep :type Boolean) (SweepResult :type Hit%20Result%20Structure%20%28by%20ref%29))
  (Utilities|FlowControl|Sequence
    (:then_0
      (bind _asbp_slime_base (Utilities|Casting|CastToBP_Slime_Base OtherActor))
      (Variables|Default|SetCharacter _asbp_slime_base)
      (Variables|Default|SetOverlap true)
      (Utilities|IsValid (Actor|GetComponentbyClass _asbp_slime_base "/Game/Code/2DMovementSystem/Component/BP_Climbing.BP_Climbing_C")
        (:Is%20Valid
          (Variables|/Game/Code/2DMovementSystem/Component/BP_Climbing.BP_Climbing_C|SetClimbThrough (Actor|GetComponentbyClass _asbp_slime_base "/Game/Code/2DMovementSystem/Component/BP_Climbing.BP_Climbing_C") (Variables|Default|GetClimbThrough))
          (Variables|/Game/Code/2DMovementSystem/Component/BP_Climbing.BP_Climbing_C|SetHorizontal (Actor|GetComponentbyClass _asbp_slime_base "/Game/Code/2DMovementSystem/Component/BP_Climbing.BP_Climbing_C") (Variables|Default|GetHorizontal)))))))

(event OnComponentEndOverlap(Box)
  (params (OverlappedComponent :type Primitive%20Component%20Object%20Reference) (OtherActor :type Actor%20Object%20Reference) (OtherComp :type Primitive%20Component%20Object%20Reference) (OtherBodyIndex :type Integer))
  (bind _asbp_slime_base (Utilities|Casting|CastToBP_Slime_Base OtherActor))
  (Variables|Default|SetCharacter _asbp_slime_base)
  (Variables|Default|SetOverlap false))

(event Custom|DetachFromLadder
  (bind _ladderparent (Variables|Default|GetLadderParent))
  (bind _character (Variables|Default|GetCharacter))
  (Utilities|IsValid _character
    (:Is%20Valid
      (Utilities|IsValid _ladderparent
        (:Is%20Valid
          (Variables|/Game/Code/2DMovementSystem/BP_Climbale/BP_Ladder.BP_Ladder_C|SetAttached _ladderparent false)
          (Transformation|DetachFromActor _character "KeepWorld" "KeepWorld" "KeepWorld"))))))

(event Custom|AttachedToLadder
  (bind _ladderparent (Variables|Default|GetLadderParent))
  (Utilities|IsValid _ladderparent
    (:Is%20Valid
      (Variables|/Game/Code/2DMovementSystem/BP_Climbale/BP_Ladder.BP_Ladder_C|SetAttached _ladderparent true))))

(event Custom|AttachedToWall
  (bind _wallparent (Variables|Default|GetWallParent))
  (Utilities|IsValid _wallparent
    (:Is%20Valid
      (Variables|/Game/Code/2DMovementSystem/BP_Climbale/BP_ClimbWall.BP_ClimbWall_C|SetAttached _wallparent true))))

(event Custom|DetachFromWall
  (bind _wallparent (Variables|Default|GetWallParent))
  (bind _character (Variables|Default|GetCharacter))
  (Utilities|IsValid _character
    (:Is%20Valid
      (Utilities|IsValid _wallparent
        (:Is%20Valid
          (Variables|/Game/Code/2DMovementSystem/BP_Climbale/BP_ClimbWall.BP_ClimbWall_C|SetAttached _wallparent false)
          (Transformation|DetachFromActor _character "KeepWorld" "KeepWorld" "KeepWorld"))))))

(event EventBeginPlay
  (bind _ladderparent (Variables|Default|GetLadderParent))
  (Utilities|IsValid _ladderparent
    (:Is%20Valid
      (Variables|Default|SetClimbThrough (Variables|/Game/Code/2DMovementSystem/BP_Climbale/BP_Ladder.BP_Ladder_C|GetClimbThrough _ladderparent)))))

(event EventTick
  (params (DeltaSeconds :type Float%20%28single-precision%29))
  (bind _wallparent (Variables|Default|GetWallParent))
  (bind _ladderparent (Variables|Default|GetLadderParent))
  (Utilities|IsValid _wallparent
    (:Is%20Valid
      (if (Variables|/Game/Code/2DMovementSystem/BP_Climbale/BP_ClimbWall.BP_ClimbWall_C|GetAttached _wallparent)
        (Utilities|IsValid (Variables|Default|GetCharacter)
          (:Is%20Valid
            (bind _output_get (Variables|Default|SetTop (Variables|/Game/Code/2DMovementSystem/BP_Climbale/BP_ClimbWall.BP_ClimbWall_C|GetTopZ _wallparent)))
            (Variables|/Game/Code/2DMovementSystem/Component/BP_Climbing.BP_Climbing_C|SetTop (Actor|GetComponentbyClass (Variables|Default|GetCharacter) "/Game/Code/2DMovementSystem/Component/BP_Climbing.BP_Climbing_C") _output_get)))))
    (:Is%20Not%20Valid
      (Utilities|IsValid _ladderparent
        (:Is%20Valid
          (if (Variables|/Game/Code/2DMovementSystem/BP_Climbale/BP_Ladder.BP_Ladder_C|GetAttached _ladderparent)
            (Utilities|IsValid (Variables|Default|GetCharacter)
              (:Is%20Valid
                (bind _output_get_2 (Variables|Default|SetTop (Variables|/Game/Code/2DMovementSystem/BP_Climbale/BP_Ladder.BP_Ladder_C|GetTopZ _ladderparent)))
                (Variables|/Game/Code/2DMovementSystem/Component/BP_Climbing.BP_Climbing_C|SetTop (Actor|GetComponentbyClass (Variables|Default|GetCharacter) "/Game/Code/2DMovementSystem/Component/BP_Climbing.BP_Climbing_C") _output_get_2)))))))))

(fn ConstructionScript
  (bind _ladderparent (Variables|Default|GetLadderParent))
  (bind _wallparent (Variables|Default|GetWallParent))
  (bind _ladderparent_2 (Variables|Default|GetLadderParent))
  (switch Utilities|FlowControl|Switch|SwitchonEnum_Climbable (Variables|Default|GetType)
    (:NewEnumerator0
      (if (Variables|Default|GetHorizontal)
        (Variables|Default|SetTypeSub (Variables|/Game/Code/2DMovementSystem/BP_Climbale/BP_Ladder.BP_Ladder_C|GetSubType _ladderparent_2))
        (Components|Box|SetBoxExtent (Variables|Default|GetBox) (Math|Vector|MakeVector 15.0 15.0 (* (Math|Conversions|ToFloat(Integer) (Variables|/Game/Code/2DMovementSystem/BP_Climbale/BP_Ladder.BP_Ladder_C|GetLength _ladderparent_2)) (/ (Variables|/Game/Code/2DMovementSystem/BP_Climbale/BP_Ladder.BP_Ladder_C|GetSectionSize _ladderparent_2) 2.3))) true)
        (else
          (Variables|Default|SetTop (Variables|/Game/Code/2DMovementSystem/BP_Climbale/BP_Ladder.BP_Ladder_C|GetTopZ _ladderparent))
          (Variables|Default|SetTypeSub (Variables|/Game/Code/2DMovementSystem/BP_Climbale/BP_Ladder.BP_Ladder_C|GetSubType (Variables|Default|GetLadderParent)))
          (Components|Box|SetBoxExtent (Variables|Default|GetBox) (Math|Vector|MakeVector 32.0 15.0 (* (Math|Conversions|ToFloat(Integer) (Variables|/Game/Code/2DMovementSystem/BP_Climbale/BP_Ladder.BP_Ladder_C|GetLength _ladderparent)) (/ (Variables|/Game/Code/2DMovementSystem/BP_Climbale/BP_Ladder.BP_Ladder_C|GetSectionSize _ladderparent) 2.3))) true))))
    (:NewEnumerator1
      (Variables|Default|SetTop (Variables|/Game/Code/2DMovementSystem/BP_Climbale/BP_ClimbWall.BP_ClimbWall_C|GetTopZ _wallparent))
      (Components|Box|SetBoxExtent (Variables|Default|GetBox) (Math|Vector|MakeVector 32.0 (* (Math|Conversions|ToFloat(Integer) (Variables|/Game/Code/2DMovementSystem/BP_Climbale/BP_ClimbWall.BP_ClimbWall_C|GetWidth _wallparent)) (/ (Variables|/Game/Code/2DMovementSystem/BP_Climbale/BP_ClimbWall.BP_ClimbWall_C|GetSectionSize _wallparent) 2.3)) (* (Math|Conversions|ToFloat(Integer) (Variables|/Game/Code/2DMovementSystem/BP_Climbale/BP_ClimbWall.BP_ClimbWall_C|GetHight _wallparent)) (/ (Variables|/Game/Code/2DMovementSystem/BP_Climbale/BP_ClimbWall.BP_ClimbWall_C|GetSectionSize _wallparent) 2.3))) true))))